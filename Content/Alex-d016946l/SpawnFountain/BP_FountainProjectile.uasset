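; BP_FountainProjectile is a homing projectile for the spawn fountain that damages the actor it is fired at.
; An init event stores the target and team ID and colors the sphere blue or red by team.
; Tick interpolates its transform toward the target, destroying it if the target is invalid.
; Any sphere overlap destroys it and applies standard damage to the stored target, whatever it overlapped.
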(event `INIT_Fountain_Projectile`
  (params (Target :type "Actor Object Reference") (Projectile_TeamID :type "/Game/c013265l/Gameplay/Enum_Teams Enum" :default "NewEnumerator0"))
  (bind _sphere (`self.Sphere`))
  ;[1 0.7921 0] Projectile Init
  (set `self.Target` Target)
  (bind _output_get (set `self.Projectile_TeamID` Projectile_TeamID))
  ;[1 1 1] Change projectile colour based on team ID
  (switch `/Game/c013265l/Gameplay/Enum_Teams` _output_get
    (:`NewEnumerator1`
      (`PrimitiveComponent.SetMaterial` _sphere 0 "/Game/A018745l/Attack_Mats/Blue_MAT.Blue_MAT"))
    (:`NewEnumerator2`
      (`PrimitiveComponent.SetMaterial` _sphere 0 "/Game/A018745l/Attack_Mats/RED_Mat.RED_Mat"))))

(event `self.ReceiveTick`
  (params (DeltaSeconds :type "Float (single-precision)"))
  ;[1 1 1] Checks if target is valid and chase it.
  (`/Engine/EditorBlueprintResources/StandardMacros.IsValid` (`self.Target`)
    (:`Is Valid`
      (`self.K2_SetActorTransform` (`KismetMathLibrary.TInterpTo` (`self.GetTransform`) (`self.GetTransform` (`self.Target`)) DeltaSeconds 10.0)))
    (:`Is Not Valid`
      (`self.K2_DestroyActor`))))

(event `self.Sphere.OnComponentBeginOverlap`
  (params (OverlappedComponent :type "PrimitiveComponent Object Reference") (OtherActor :type "Actor Object Reference") (OtherComp :type "PrimitiveComponent Object Reference") (OtherBodyIndex :type Integer) (bFromSweep :type Boolean) (SweepResult :type "HitResult Structure (by ref)"))
  ;[1 1 1] On contact with the target
  (`self.K2_DestroyActor`)
  (`GameplayStatics.ApplyDamage` (`self.Target`) 10.0 null null "/Game/c013265l/Blueprints/DamageTypes/BP_StandardDamage.BP_StandardDamage_C"))

(fn `UserConstructionScript`)
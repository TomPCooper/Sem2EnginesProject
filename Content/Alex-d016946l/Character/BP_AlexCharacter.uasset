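; BP_AlexCharacter is a team-coloured sledgehammer fighter with a basic melee attack and three abilities.
; Each action plays a montage and checks AbilityInUse, though Guard never sets it.
; Basic attack and Ground Slam apply sphere-trace damage after delays, while Guard slows movement and sets Blocking for the parent class.
; Circle Hammer hides the held hammer and uses a timeline to move a spawned BP_SledgeHammer along a spline.
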(event `self.ReceiveBeginPlay`
  (bind _hammer_head (`self.Hammer_Head`))
  ;[1 1 1] On begin play set the head of the sledgehammer's colour to blue or read depending on team ID
  (switch `/Game/c013265l/Gameplay/Enum_Teams` (`self.Team ID`)
    (:`NewEnumerator1`
      (`PrimitiveComponent.SetMaterial` _hammer_head 0 "/Game/A018745l/Attack_Mats/Blue_MAT.Blue_MAT"))
    (:`NewEnumerator2`
      (`PrimitiveComponent.SetMaterial` _hammer_head 0 "/Game/A018745l/Attack_Mats/RED_Mat.RED_Mat"))))

(event `self.FireBasicAttack`
  ;[1 1 1] Basic Attack
  (if (not (`self.Ability in use`))
    (set `self.Ability in use` true)
    ;;[0.04025 1 0.9502] Play animation
    (`|PlayMontage` (`self.Mesh`) "/Game/Alex-d016946l/Character/Assets/animations/Great_Sword_Slash_Montage.Great_Sword_Slash_Montage"
      (:`then`
        (`KismetSystemLibrary.Delay` 0.8)
        (set `self.Ability in use` false)
        (bind (_outhit _returnvalue) (`KismetSystemLibrary.SphereTraceSingleForObjects` (`self.K2_GetActorLocation`) (`SceneComponent.K2_GetComponentLocation` (`self.Basic_Attack_point`)) 80.0 (`|MakeArray` "ObjectTypeQuery3" :!type "EObjectTypeQuery Enum")))
        (if _returnvalue
          (`GameplayStatics.ApplyDamage` (`.HitActor` (`GameplayStatics.BreakHitResult` _outhit)) 15.0 (`self.GetController`) null "/Game/c013265l/Blueprints/DamageTypes/BP_StandardDamage.BP_StandardDamage_C"))))))

(event `self.FireAbility1`
  (bind _returnvalue (`self.K2_GetActorLocation`))
  (bind _capsulecomponent (`self.CapsuleComponent`))
  ;[1 1 1] Ability 1 - Ground Slam
  (if (not (`self.Ability in use`))
    (set `self.Ability in use` true)
    ;;[1 0 0] Disable Input
    (`self.DisableInput` (`GameplayStatics.GetPlayerController` 0))
    ;;[0.04025 1 0.9502] Play animation
    (`|PlayMontage` (`self.Mesh`) "/Game/Alex-d016946l/Character/Assets/animations/Jump_Attack_Montage.Jump_Attack_Montage"
      (:`then`
        (`self.LaunchCharacter` (+ (+ (* (`SceneComponent.GetForwardVector` _capsulecomponent) 100.0) (* (`SceneComponent.GetRightVector` _capsulecomponent) 1.0)) (* (`SceneComponent.GetUpVector` _capsulecomponent) 5.0)))
        (`KismetSystemLibrary.Delay` 1.3)
        (set `self.Ability in use` false)
        (`self.EnableInput` (`GameplayStatics.GetPlayerController` 0))
        (bind _outhits (`KismetSystemLibrary.SphereTraceMultiForObjects` _returnvalue _returnvalue 200.0 (`|MakeArray` "ObjectTypeQuery3" :!type "EObjectTypeQuery Enum")))
        (if true
          (for _array_element _outhits
            (`GameplayStatics.ApplyDamage` (`.HitActor` (`GameplayStatics.BreakHitResult` _array_element)) 40.0 (`self.GetController`) null "/Game/c013265l/Blueprints/DamageTypes/BP_StandardDamage.BP_StandardDamage_C")))))))

(event `self.FireAbility2`
  ;[1 1 1] Ability 2 - Guard (The actual function is done in the parent class on any damage event) It divides the damage received by 2
  (if (not (`self.Ability in use`))
    ;;[0.04025 1 0.9502] Play animation
    (`|PlayMontage` (`self.Mesh`) "/Game/Alex-d016946l/Character/Assets/animations/Standing_Block_Idle_Montage.Standing_Block_Idle_Montage"
      (:`then`
        (set `CharacterMovementComponent.MaxWalkSpeed` 200.0 (`self.CharacterMovement`))
        (set `self.blocking` true)
        (`KismetSystemLibrary.Delay` 1.0)
        (set `self.Ability in use` false)
        (set `self.blocking` false)
        (set `CharacterMovementComponent.MaxWalkSpeed` 500.0 (`self.CharacterMovement`))))))

(event `self.FireAbility3`
  (bind _spline (`self.Spline`))
  ;[1 1 1] Ability 3: Circle Hammer
  (if (not (`self.Ability in use`))
    (set `self.Ability in use` true)
    ;;[1 0 0] Disable Input
    (`self.DisableInput` (`GameplayStatics.GetPlayerController` 0))
    ;;[0.04025 1 0.9502] Play animation
    (`|PlayMontage` (`self.Mesh`) "/Game/Alex-d016946l/Character/Assets/animations/Great_Sword_Slash_Montage.Great_Sword_Slash_Montage"
      (:`then`
        ;;[1 0.6879 0.1183] After delay, it sets visiblity of the hammer in hand to invisible
        (`KismetSystemLibrary.Delay` 0.8)
        (`SceneComponent.SetVisibility` (`self.Hammer_Handle`) false false)
        (`SceneComponent.SetVisibility` (`self.Hammer_Head`) false false)
        (`self.EnableInput` (`GameplayStatics.GetPlayerController` 0))
        ;;[1 0.7225 0.1718] Spawn another hammer to rotate around player
        (bind _returnvalue (`|SpawnActorFromClass` "/Game/Alex-d016946l/Character/BP_SledgeHammer.BP_SledgeHammer_C" (`SceneComponent.GetRelativeTransform` (`self.Basic_Attack_point`)) "AlwaysSpawn" "OverrideRootScale" null null))
        (bind _output_get (set `self.Thrown_SledgeHammer_ref` _returnvalue))
        (`/Game/Alex-d016946l/Character/BP_SledgeHammer.INIT_thrownHammer` _output_get (`self.Team ID`) (`self.GetController`))
        ;;[1 0.7465 0.04235] Rotate the hammer around the spline
        (bind (_direction _newtrack_0) (`Timeline|Move_SledgeHammer` :!via `PlayFromStart`)
          (:`Update`
            (bind _returnvalue_2 (`KismetMathLibrary.Lerp` 0.0 (`SplineComponent.GetSplineLength` (`self.Spline`)) _newtrack_0))
            (`self.K2_SetActorTransform` (`self.Thrown_SledgeHammer_ref`) (`KismetMathLibrary.MakeTransform` (`SplineComponent.GetLocationAtDistanceAlongSpline` _spline _returnvalue_2 "World") (`SplineComponent.GetRotationAtDistanceAlongSpline` _spline _returnvalue_2 "World")) false false))
          (:`Finished`
            (`self.K2_DestroyActor` (`self.Thrown_SledgeHammer_ref`))
            (`SceneComponent.SetVisibility` (`self.Hammer_Handle`) true false)
            (`SceneComponent.SetVisibility` (`self.Hammer_Head`) true false)
            (set `self.Ability in use` false)))))))

(fn `UserConstructionScript`
  (`parent.UserConstructionScript`))
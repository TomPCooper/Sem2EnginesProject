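; BP_SledgeHammer is a thrown hammer that spins and damages actors it overlaps, then destroys itself after ten seconds.
; INIT_thrownHammer stores the owning controller and colours the head blue or red by team.
; A timeline started on BeginPlay rolls the capsule for the spin.
; Capsule overlaps apply standard damage with the owner as instigator, leaving friendly-fire filtering to the damage receiver's health logic.
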(event `INIT_thrownHammer`
  (params (TeamID :type "/Game/c013265l/Gameplay/Enum_Teams Enum" :default "NewEnumerator0") (Owner_Controller :type "Controller Object Reference"))
  (bind _hammer_head (`self.Hammer_Head`))
  ;[1 1 1] Setting the head of the hammer to red or blue based on team ID
  (set `self.Owner Controller` Owner_Controller)
  (switch `/Game/c013265l/Gameplay/Enum_Teams` TeamID
    (:`NewEnumerator1`
      (`PrimitiveComponent.SetMaterial` _hammer_head 0 "/Game/A018745l/Attack_Mats/Blue_MAT.Blue_MAT"))
    (:`NewEnumerator2`
      (`PrimitiveComponent.SetMaterial` _hammer_head 0 "/Game/A018745l/Attack_Mats/RED_Mat.RED_Mat"))))

(event `self.ReceiveBeginPlay`
  ;[1 1 1] The rotating animation is done here
  (`KismetSystemLibrary.K2_SetTimerDelegate` (delegate `Destroy hammer after 10 seconds`) 10.0)
  (bind (_direction _speed) (`Timeline|Rotation_Animation`)
    (:`Update`
      (bind _returnvalue_roll (`KismetMathLibrary.BreakRotator` (`KismetMathLibrary.RLerp` (`KismetMathLibrary.MakeRotator` 0.0) (`KismetMathLibrary.MakeRotator` 360.0) _speed)))
      (`SceneComponent.K2_SetRelativeRotation` (`self.Capsule`) (`KismetMathLibrary.MakeRotator` _returnvalue_roll 90.0) false false))))

(event `Destroy hammer after 10 seconds`
  ;[1 1 1] The rotating animation is done here
  (`self.K2_DestroyActor`))

(event `self.Capsule.OnComponentBeginOverlap`
  (params (OverlappedComponent :type "PrimitiveComponent Object Reference") (OtherActor :type "Actor Object Reference") (OtherComp :type "PrimitiveComponent Object Reference") (OtherBodyIndex :type Integer) (bFromSweep :type Boolean) (SweepResult :type "HitResult Structure (by ref)"))
  ;[1 1 1] On contact Apply damage. (I don't need to get Team ID here because of the modify health logic from the parent class on any damage). If given the controller the game can identify which attack is friendly and neglect it.
  (`GameplayStatics.ApplyDamage` OtherActor 10.0 (`self.Owner Controller`) null "/Game/c013265l/Blueprints/DamageTypes/BP_StandardDamage.BP_StandardDamage_C"))

(fn `UserConstructionScript`)
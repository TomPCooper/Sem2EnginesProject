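; BP_MinionAI is the AI controller for minions, starting their behavior tree on BeginPlay.
; It finds the BP_ControlPoint actor, prints the controlled pawn's name, then runs BT_Minion with the BB_Minion blackboard.
; It seeds that blackboard with the control point's location and a fixed detection radius for the tree to use.
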(event `self.ReceiveBeginPlay`
  (`|ExecutionSequence`
    (:`then_0`
      (bind _returnvalue (`GameplayStatics.GetActorOfClass` "/Game/Alex-d016946l/ControlPoint/BP_ControlPoint.BP_ControlPoint_C"))
      (set `self.ControlPoint_ref` _returnvalue))
    (:`then_1`
      (`KismetSystemLibrary.PrintString` (`KismetSystemLibrary.GetDisplayName` (`self.K2_GetPawn`)))
      (`self.RunBehaviorTree` "/Game/Alex-d016946l/Minions/BT_Minion.BT_Minion")
      (bind _blackboardcomponent (`self.UseBlackboard` "/Game/Alex-d016946l/Minions/BB_Minion.BB_Minion"))
      (bind _output_get (set `self.Blackboard Component` _blackboardcomponent))
      (`|ExecutionSequence`
        (:`then_0`
          (`BlackboardComponent.SetValueAsVector` _output_get "ControlPoint" (`self.K2_GetActorLocation` (`self.ControlPoint_ref`))))
        (:`then_1`
          (`BlackboardComponent.SetValueAsFloat` _output_get "DetectionRadius" 300.0))))))

(fn `UserConstructionScript`)
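; Team-based minion that attacks actors entering its box and can be damaged, healed or killed.
; Box overlap sets the target and starts a looping timer that applies standard damage; ending overlap stops it.
; AnyDamage branches on damage type class name: teammates' healing restores health, and their standard damage is halved.
; Team IDs come from controllers through interface messages, while health changes update a widget bar and depletion destroys the actor.
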(event `self.ReceiveBeginPlay`
  (`KismetSystemLibrary.K2_ClearAndInvalidateTimerHandle` (`self.AttackTimer_Handle`)))

(event `INIT_MinionBP`
  ;[1 1 1] INIT
  (bind _teamid (message `/Game/c013265l/Blueprints/Interfaces/BPI_Teams.I_GetTeam` (`self.GetController`)))
  (set `self.BPminion_TeamID` _teamid)
  (`TextRenderComponent.K2_SetText` (`self.Minion TeamID Text`) (`KismetTextLibrary.Conv_StringToText` (`|GetEnumeratorNameAsString` (`self.BPminion_TeamID`))))
  (`TextRenderComponent.SetTextRenderColor` (`self.Minion TeamID Text`) (select `/Game/c013265l/Gameplay/Enum_Teams` (`self.BPminion_TeamID`) :`NewEnumerator0` (make `Color` :`G` 255) :`NewEnumerator1` (make `Color` :`B` 255) :`NewEnumerator2` (make `Color` :`R` 255))))

(event `Set Attack Timer`
  (bind _returnvalue (`KismetSystemLibrary.K2_SetTimer` null "StartAttack" 1.0 true))
  (set `self.AttackTimer_Handle` _returnvalue))

(event `self.Box.OnComponentBeginOverlap`
  (params (OverlappedComponent :type "PrimitiveComponent Object Reference") (OtherActor :type "Actor Object Reference") (OtherComp :type "PrimitiveComponent Object Reference") (OtherBodyIndex :type Integer) (bFromSweep :type Boolean) (SweepResult :type "HitResult Structure (by ref)"))
  (set `self.Attack_Counter` 0)
  (set `self.Target` OtherActor)
  (`self.Set Attack Timer`))

(event `Player Out Of Range`
  (`KismetSystemLibrary.K2_ClearAndInvalidateTimerHandle` (`self.AttackTimer_Handle`)))

(event `self.Box.OnComponentEndOverlap`
  (params (OverlappedComponent :type "PrimitiveComponent Object Reference") (OtherActor :type "Actor Object Reference") (OtherComp :type "PrimitiveComponent Object Reference") (OtherBodyIndex :type Integer))
  (set `self.Target` null)
  (`self.Player Out Of Range`))

(event `self.ReceiveAnyDamage`
  (params (Damage :type "Float (single-precision)") (DamageType :type "DamageType Object Reference") (InstigatedBy :type "Controller Object Reference") (DamageCauser :type "Actor Object Reference"))
  ;[1 0.257 0.08683] Event Any Damage with friendly fire check
  (switch `string` (`KismetSystemLibrary.GetClassDisplayName` (`GameplayStatics.GetObjectClass` DamageType))
    (:`BP_HealingDamage_C`
      ;;[1 1 1] This friendly fire check is used to check if it's a team mate, if yes it gets healed, if it's an enemy,  nothing happens
      (bind _friend_ (`self.Friendly Fire Check` InstigatedBy))
      (if _friend_
        (set `self.Health` (+ (`self.Health`) Damage))
        (bind _aswbp_minion_health_bar (cast `/Game/Alex-d016946l/Minions/WBP_Minion_HealthBar` (`WidgetComponent.GetUserWidgetObject` (`self.Widget_HealthBar`))))
        (`ProgressBar.SetPercent` (`/Game/Alex-d016946l/Minions/WBP_Minion_HealthBar.BarProgress_HealthBar` _aswbp_minion_health_bar) (/ (`self.Health`) 100.0))))
    (:`BP_StandardDamage_C`
      ;;[1 1 1] This friendly fire is used to check if it's a team mate, if yes it diminishes the damage by half, if it's an enemy, it takes full damage
      (bind _friend__2 (`self.Friendly Fire Check` InstigatedBy))
      (if _friend__2
        (bind _output_get (set `self.Health` (- (`self.Health`) (/ Damage 2.0))))
        (if (<= _output_get 0.0)
          (`self.K2_DestroyActor`)
          (else
            (bind _aswbp_minion_health_bar_2 (cast `/Game/Alex-d016946l/Minions/WBP_Minion_HealthBar` (`WidgetComponent.GetUserWidgetObject` (`self.Widget_HealthBar`))))
            (`ProgressBar.SetPercent` (`/Game/Alex-d016946l/Minions/WBP_Minion_HealthBar.BarProgress_HealthBar` _aswbp_minion_health_bar_2) (/ (`self.Health`) 100.0))))
        (else
          (bind _output_get_2 (set `self.Health` (- (`self.Health`) Damage)))
          (if (<= _output_get_2 0.0)
            (`self.K2_DestroyActor`)
            (else
              (bind _aswbp_minion_health_bar_3 (cast `/Game/Alex-d016946l/Minions/WBP_Minion_HealthBar` (`WidgetComponent.GetUserWidgetObject` (`self.Widget_HealthBar`))))
              (`ProgressBar.SetPercent` (`/Game/Alex-d016946l/Minions/WBP_Minion_HealthBar.BarProgress_HealthBar` _aswbp_minion_health_bar_3) (/ (`self.Health`) 100.0)))))))))

(fn `Friendly Fire Check`
  (params (InstigatorController :type "Object Object Reference"))
  (returns (`Friend?` :type Boolean))
  ;[1 1 1] This function is used to compare the instigator team ID to the minion TeamID
  (`/Engine/EditorBlueprintResources/StandardMacros.IsValid` InstigatorController
    (:`Is Valid`
      (bind _teamid (message `/Game/c013265l/Blueprints/Interfaces/BPI_Teams.I_GetTeam` (`self.GetController`)))
      (bind _teamid_2 (message `/Game/c013265l/Blueprints/Interfaces/BPI_Teams.I_GetTeam` InstigatorController))
      (if (`|EnumEquality` _teamid_2 _teamid)
        (return true)
        (else
          _)))
    (:`Is Not Valid`
      _))
  (return false))

(fn `I_GetPlayerData`
  (returns (PlayerData :type "/Game/c013265l/Structs/S_PlayerData Structure"))
  (return))

(fn `I_GetTeam`
  (returns (TeamID :type "/Game/c013265l/Gameplay/Enum_Teams Enum"))
  (bind _teamid (message `/Game/c013265l/Blueprints/Interfaces/BPI_Teams.I_GetTeam` (`self.GetController`)))
  (return _teamid))

(fn `StartAttack`
  (`GameplayStatics.ApplyDamage` (`self.Target`) 25.0 (`self.GetController`) self "/Game/c013265l/Blueprints/DamageTypes/BP_StandardDamage.BP_StandardDamage_C")
  (bind _result (`/Engine/EditorBlueprintResources/StandardMacros.IncrementInt` (`self.Attack_Counter`))
    (:`  `
      (`KismetSystemLibrary.PrintString` (`KismetStringLibrary.Concat_StrStr` (`KismetStringLibrary.Concat_StrStr` (`KismetSystemLibrary.GetDisplayName` (`self.GetController`))) "  Attack no:  " (`KismetStringLibrary.Conv_IntToString` _result)) true false (struct :`G` 0.66 :`B` 1.0 :`A` 1.0) 0.999))))

(fn `UserConstructionScript`)
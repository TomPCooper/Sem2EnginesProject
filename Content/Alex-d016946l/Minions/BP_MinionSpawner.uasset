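; BP_MinionSpawner is a spawner actor that produces team-assigned BP_Minion units at its own transform.
; Custom events start and clear a looping one-second timer on MinionSpawn; BeginPlay does not start it.
; While Active, each tick of that timer spawns a minion, sends SpawnerTeamID to its controller by interface message, then initialises it.
; The construction script sets the MinionSpawner text colour from the team ID.
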(event `self.ReceiveBeginPlay`)

(event `Set_Timer_MinionSpawn`
  ;[1 1 1] Spawn minions every one second and initialise them
  (bind _returnvalue (`KismetSystemLibrary.K2_SetTimer` null "MinionSpawn" 1.0 true))
  (set `self.MinionSpawn_Handle` _returnvalue))

(event `Clear_Handle_MinionSpawn`
  ;[1 1 1] Stop spawning
  (`KismetSystemLibrary.K2_ClearAndInvalidateTimerHandle` (`self.MinionSpawn_Handle`)))

(fn `MinionSpawn`
  (if (`self.Active?`)
    (bind _returnvalue (`|SpawnActorFromClass` "/Game/Alex-d016946l/Minions/BP_Minion.BP_Minion_C" (`self.GetTransform`) "AdjustIfPossibleButAlwaysSpawn" "OverrideRootScale" null null))
    (message `/Game/c013265l/Blueprints/Interfaces/BPI_Teams.I_SetTeam` (`Pawn.GetController` _returnvalue) (`self.Spawner_TeamID`))
    (`/Game/Alex-d016946l/Minions/BP_Minion.INIT_MinionBP` _returnvalue)))

(fn `UserConstructionScript`
  (`TextRenderComponent.SetTextRenderColor` (`self.MinionSpawner`) (select `/Game/c013265l/Gameplay/Enum_Teams` (`self.Spawner_TeamID`) :`NewEnumerator0` (make `Color` :`G` 255) :`NewEnumerator1` (make `Color` :`B` 255) :`NewEnumerator2` (make `Color` :`R` 255))))
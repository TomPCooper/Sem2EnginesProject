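; Manager for a King of the Hill control point that scores two teams and tracks round wins.
; Events start and stop per-team timelines, which drive progress, percentage and time-left widgets in the KOTH UI.
; A finished timeline adds a round win, updates win textures and stops the point's tick; only Team B's also notifies GM_KOTHbad.
; An end-game check treats two wins as victory, only printing the result.
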(event `init_ControlPoint_M`
  (params (ui_KOTH :type "/Game/Alex-d016946l/Alex_GameModes/UI_KOTH Object Reference") (BP_ControlPoint :type "/Game/Alex-d016946l/ControlPoint/BP_ControlPoint Object Reference"))
  ;[1 0.6431 0] Init
  (bind _output_get (set `self.Ui KOTH` ui_KOTH))
  (`KismetSystemLibrary.PrintString` "MANAGER INITIATED" true true (struct :`R` 0.190076 :`G` 1.0 :`A` 1.0) 10.0)
  (`/Game/Alex-d016946l/Alex_GameModes/UI_KOTH.Init_Texture` _output_get "/Game/Alex-d016946l/ControlPoint/Materials_and_textures/ControlPointYellow.ControlPointYellow")
  (set `self.ControlPoint_ref` BP_ControlPoint))

(event `Increasing score Team_A`
  (bind _ui_koth (`self.Ui KOTH`))
  ;[1 1 1] When the control point is captured, it will increase the score for the team
  (bind (_direction _team_a_progress _team_a_seconds_left) (`Timeline|Team A score` :!label _label)
    (:`Update`
      (`ProgressBar.SetPercent` (`/Game/Alex-d016946l/Alex_GameModes/UI_KOTH.ProgressBar_TeamA` (`self.Ui KOTH`)) _team_a_progress)
      (set `TextBlock.Text` (`KismetTextLibrary.Conv_DoubleToText` (* _team_a_progress 100.0) "HalfToEven") (`/Game/Alex-d016946l/Alex_GameModes/UI_KOTH.Text_Percentage_TeamA` _ui_koth))
      (set `TextBlock.Text` (`KismetTextLibrary.Conv_DoubleToText` _team_a_seconds_left "HalfToEven") (`/Game/Alex-d016946l/Alex_GameModes/UI_KOTH.Text_TimeLeft_TeamA` _ui_koth)))
    (:`Finished`
      (`KismetSystemLibrary.PrintString` "TEAM A WON" true true (struct :`G` 0.029324 :`B` 1.0 :`A` 1.0) 10.0)
      (bind _result (`/Engine/EditorBlueprintResources/StandardMacros.IncrementInt` (`self.RoundsWon_TeamA`))
        (:`  `
          (`/Game/Alex-d016946l/Alex_GameModes/UI_KOTH.Get_Texture` (`self.Ui KOTH`) (`self.Blue_Texture`) _result true)
          (`self.SetActorTickEnabled` (`self.ControlPoint_ref`) false))))))

(event `Stop Scoring Team_A`
  ;[1 1 1] When the control point is captured, it will increase the score for the team
  (goto _label :!via `Stop`))

(event `Stop Scoring Team_Both`
  (bind _ui_koth (`self.Ui KOTH`))
  ;[1 1 1] When the control point is captured, it will increase the score for the team
  (`|ExecutionSequence`
    (:`then_0`
      (goto _label :!via `Stop`))
    (:`then_1`
      (bind (_direction _team_b_progress _team_b_seconds_left) (`Timeline|Team B Score` :!via `Stop` :!label _label_2)
        (:`Update`
          (`ProgressBar.SetPercent` (`/Game/Alex-d016946l/Alex_GameModes/UI_KOTH.ProgressBar_TeamB` (`self.Ui KOTH`)) _team_b_progress)
          (set `TextBlock.Text` (`KismetTextLibrary.Conv_DoubleToText` (* _team_b_progress 100.0) "HalfToEven") (`/Game/Alex-d016946l/Alex_GameModes/UI_KOTH.Text_Percentage_TeamB` _ui_koth))
          (set `TextBlock.Text` (`KismetTextLibrary.Conv_DoubleToText` _team_b_seconds_left "HalfToEven") (`/Game/Alex-d016946l/Alex_GameModes/UI_KOTH.Text_TimeLeft_TeamB` _ui_koth)))
        (:`Finished`
          (`KismetSystemLibrary.PrintString` "TEAM B won the round!" true true (struct :`R` 1.0 :`B` 0.042985 :`A` 1.0) 10.0)
          (bind _result (`/Engine/EditorBlueprintResources/StandardMacros.IncrementInt` (`self.RoundsWon_TeamB`))
            (:`  `
              (`/Game/Alex-d016946l/Alex_GameModes/UI_KOTH.Get_Texture` (`self.Ui KOTH`) (`self.Red_Texture`) _result false)
              (`self.SetActorTickEnabled` (`self.ControlPoint_ref`) false)
              (`/Game/Alex-d016946l/Alex_GameModes/GM_KOTHbad.GameStateChanged` (cast `/Game/Alex-d016946l/Alex_GameModes/GM_KOTHbad` (`GameplayStatics.GetGameMode`) :!pure true) "NewEnumerator3"))))))))

(event `Increasing score Team_B`
  ;[1 1 1] When the control point is captured, it will increase the score for the team
  (goto _label_2))

(event `Stop Scoring Team_B`
  ;[1 1 1] When the control point is captured, it will increase the score for the team
  (goto _label_2 :!via `Stop`))

(event `EndGame who won`
  (bind _team (`self.Can End Game & Who Won` (`self.RoundsWon_TeamA`) (`self.RoundsWon_TeamB`)))
  (if (== _team 0)
    (`KismetSystemLibrary.PrintString` "No one won yet, beginning new round..." true true (struct :`R` 0.09145 :`G` 1.0 :`A` 1.0) 6.0)
    (elif (== _team 1)
      (`KismetSystemLibrary.PrintString` " \n \nTeam Blue WON!! \n \n" true true (struct :`R` 0.023822 :`B` 1.0 :`A` 1.0) 6.0)
      (elif (== _team 2)
        (`KismetSystemLibrary.PrintString` " \n \nTeam Red WON!! \n \n" true true (struct :`R` 0.023822 :`B` 1.0 :`A` 1.0) 6.0)))))

(fn `Can End Game & Who Won`
  (params (RoundsWon_TeamA :type Integer) (RoundsWon_TeamB :type Integer))
  (returns (Team :type Integer))
  (if (== RoundsWon_TeamA 2)
    (return 1)
    (elif (== RoundsWon_TeamB 2)
      (return 2)
      (else
        (`KismetSystemLibrary.PrintString` "No One Won")
        (return 0)))))

(fn `UserConstructionScript`)
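; King of the Hill manager that tracks and displays capture-point scoring for Team A and Team B.
; It receives the KOTH widget on init, then start and stop events control a separate score timeline per team.
; Timeline tracks drive each team's progress bar, percentage and time-left text, with stopping halting playback in place.
; A finished timeline only prints that team's win message.
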(event `init_Manager`
  (params (ui_KOTH :type "/Game/Alex-d016946l/Alex_GameModes/UI_KOTH Object Reference") (GS_GameState :type Boolean))
  (set `self.Ui KOTH` ui_KOTH)
  (`KismetSystemLibrary.PrintString` "MANAGER INITIATED" true true (struct :`R` 0.190076 :`G` 1.0 :`A` 1.0) 10.0))

(event `Increasing score Team_A`
  (bind _ui_koth (`self.Ui KOTH`))
  ;[1 1 1] When the control point is captured, it will increase the score for the team
  (bind (_direction _team_a_progress _team_a_seconds_left) (`Timeline|Team A score` :!label _label)
    (:`Update`
      (`ProgressBar.SetPercent` (`/Game/Alex-d016946l/Alex_GameModes/UI_KOTH.ProgressBar_TeamA` (`self.Ui KOTH`)) _team_a_progress)
      (set `TextBlock.Text` (`KismetTextLibrary.Conv_DoubleToText` (* _team_a_progress 100.0) "HalfToEven") (`/Game/Alex-d016946l/Alex_GameModes/UI_KOTH.Text_Percentage_TeamA` _ui_koth))
      (set `TextBlock.Text` (`KismetTextLibrary.Conv_DoubleToText` _team_a_seconds_left "HalfToEven") (`/Game/Alex-d016946l/Alex_GameModes/UI_KOTH.Text_TimeLeft_TeamA` _ui_koth)))
    (:`Finished`
      (`KismetSystemLibrary.PrintString` "TEAM A WON" true true (struct :`G` 0.029324 :`B` 1.0 :`A` 1.0) 10.0))))

(event `Stop Scoring Team_A`
  ;[1 1 1] When the control point is captured, it will increase the score for the team
  (goto _label :!via `Stop`))

(event `Stop Scoring Team_Both`
  (bind _ui_koth (`self.Ui KOTH`))
  ;[1 1 1] When the control point is captured, it will increase the score for the team
  (`|ExecutionSequence`
    (:`then_0`
      (goto _label :!via `Stop`))
    (:`then_1`
      (bind (_direction _team_b_progress _team_b_seconds_left) (`Timeline|Team B Score` :!via `Stop` :!label _label_2)
        (:`Update`
          (`ProgressBar.SetPercent` (`/Game/Alex-d016946l/Alex_GameModes/UI_KOTH.ProgressBar_TeamB` (`self.Ui KOTH`)) _team_b_progress)
          (set `TextBlock.Text` (`KismetTextLibrary.Conv_DoubleToText` (* _team_b_progress 100.0) "HalfToEven") (`/Game/Alex-d016946l/Alex_GameModes/UI_KOTH.Text_Percentage_TeamB` _ui_koth))
          (set `TextBlock.Text` (`KismetTextLibrary.Conv_DoubleToText` _team_b_seconds_left "HalfToEven") (`/Game/Alex-d016946l/Alex_GameModes/UI_KOTH.Text_TimeLeft_TeamB` _ui_koth)))
        (:`Finished`
          (`KismetSystemLibrary.PrintString` "TEAM B WON" true true (struct :`R` 1.0 :`B` 0.042985 :`A` 1.0) 10.0))))))

(event `Increasing score Team_B`
  ;[1 1 1] When the control point is captured, it will increase the score for the team
  (goto _label_2))

(event `Stop Scoring Team_B`
  ;[1 1 1] When the control point is captured, it will increase the score for the team
  (goto _label_2 :!via `Stop`))

(fn `UserConstructionScript`)
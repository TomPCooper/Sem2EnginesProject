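; King of the Hill game mode that sets up a local multiplayer match with two teams.
; On BeginPlay it replaces the default player with local players numbered by the PlayerCount option, alternating teams via FlipFlop and interface messages.
; It spawns a colored character per controller at a random BP_TeamPlayerStart matching its team, then possesses it.
; Controller and team lists track membership through login and logout; the ChoosePlayerStart override is empty.
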(event `self.ReceiveBeginPlay`
  (`self.SetUpController` (`GameplayStatics.GetIntOption` (`self.OptionsString`) "PlayerCount"))
  (`self.SpawnCharacters`))

(event `self.K2_PostLogin`
  (params (NewPlayer :type "PlayerController Object Reference"))
  (bind _aspc_game (cast `/Game/c013265l/Blueprints/PlayerControllers/PC_Game` NewPlayer))
  (`KismetArrayLibrary.Array_Add` (`self.GamePlayControllers`) _aspc_game))

(event `self.K2_OnLogout`
  (params (ExitingController :type "Controller Object Reference"))
  (bind _aspc_game (cast `/Game/c013265l/Blueprints/PlayerControllers/PC_Game` ExitingController))
  (`KismetArrayLibrary.Array_RemoveItem` (`self.GamePlayControllers`) _aspc_game)
  (`KismetArrayLibrary.Array_RemoveItem` (`self.TeamA_Players`) _aspc_game)
  (`KismetArrayLibrary.Array_RemoveItem` (`self.TeamB_Players`) _aspc_game))

(fn `AddToTeamLists`
  (params (GameplayController :type "/Game/c013265l/Blueprints/PlayerControllers/PC_Game Object Reference"))
  (bind _teamid (message `/Game/c013265l/Blueprints/Interfaces/BPI_Teams.I_GetTeam` GameplayController))
  (switch `/Game/c013265l/Gameplay/Enum_Teams` _teamid
    (:`NewEnumerator1`
      (`KismetArrayLibrary.Array_Add` (`self.TeamA_Players`) GameplayController))
    (:`NewEnumerator2`
      (`KismetArrayLibrary.Array_Add` (`self.TeamB_Players`) GameplayController))))

(fn `ChoosePlayerStart`
  (params (Player :type "Controller Object Reference"))
  (returns (ReturnValue :type "Actor Object Reference"))
  (return null))

(fn `SelectPlayerStart`
  (params (TeamID :type "/Game/c013265l/Gameplay/Enum_Teams Enum" :default "NewEnumerator0"))
  (returns (StartActor :type "/Game/c013265l/Gameplay/BP_TeamPlayerStart Object Reference"))
  (locals (L_SpawnPointActors :type "Array of /Game/c013265l/Gameplay/BP_TeamPlayerStart Object Reference"))
  (bind _outactors (`GameplayStatics.GetAllActorsOfClass` "/Game/c013265l/Gameplay/BP_TeamPlayerStart.BP_TeamPlayerStart_C"))
  (for _array_element _outactors
    (bind _teamid (message `/Game/c013265l/Blueprints/Interfaces/BPI_Teams.I_GetTeam` _array_element))
    (if (`|EnumEquality` _teamid TeamID)
      (`KismetArrayLibrary.Array_Add` (`local.L_SpawnPointActors`) _array_element)))
  (if (!= (`KismetArrayLibrary.Array_Length` (`local.L_SpawnPointActors`)) 0)
    (return (`KismetArrayLibrary.Array_Random` (`local.L_SpawnPointActors`)))
    (else
      (bind _returnvalue (`GameplayStatics.GetActorOfClass` "/Game/c013265l/Gameplay/BP_TeamPlayerStart.BP_TeamPlayerStart_C"))
      (return _returnvalue))))

(fn `SetUpController`
  (params (PlayerCount :type Integer))
  (`GameplayStatics.RemovePlayer` (`GameplayStatics.GetPlayerController` 0) true)
  (for _index (range PlayerCount)
    (bind _returnvalue (`GameplayStatics.CreatePlayer` _index))
    (`/Engine/EditorBlueprintResources/StandardMacros.FlipFlop`
      (:`A`
        (message `/Game/c013265l/Blueprints/Interfaces/BPI_Teams.I_SetTeam` _returnvalue "NewEnumerator1"))
      (:`B`
        (message `/Game/c013265l/Blueprints/Interfaces/BPI_Teams.I_SetTeam` _returnvalue "NewEnumerator2")))
    (`self.AddToTeamLists` (cast `/Game/c013265l/Blueprints/PlayerControllers/PC_Game` _returnvalue :!pure true))))

(fn `SpawnCharacters`
  (for (_array_element _array_index) (`self.GamePlayControllers`)
    (bind _teamid (message `/Game/c013265l/Blueprints/Interfaces/BPI_Teams.I_GetTeam` _array_element))
    (bind _returnvalue (`|SpawnActorFromClass` (select `int` _array_index :`0` "/Game/c013265l/Characters/BP_Char_Blue.BP_Char_Blue_C" :`1` "/Game/c013265l/Characters/BP_Char_Green.BP_Char_Green_C" :`2` "/Game/c013265l/Characters/BP_Char_Red.BP_Char_Red_C" :`3` "/Game/c013265l/Characters/BP_ThirdPersonCharacter_Yellow.BP_ThirdPersonCharacter_Yellow_C" :!type "/Game/ThirdPerson/Blueprints/BP_ThirdPersonCharacter Class Reference") (`self.GetTransform` (`self.SelectPlayerStart` _teamid)) "AdjustIfPossibleButAlwaysSpawn" "OverrideRootScale" null null))
    (`Controller.Possess` _array_element (cast `Pawn` _returnvalue :!pure true))))

(fn `UserConstructionScript`)
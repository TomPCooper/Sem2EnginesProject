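; King of the Hill manager Blueprint that runs team scoring for a control point and decides when a round is won.
; Events play or stop one timeline per team, so progress resumes where it stopped and drives that team's UI progress bar and time-left text.
; A finished timeline increments that team's wins, updates the UI, disables the point's tick, notifies the game mode and rewinds both timelines.
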(event `init_ControlPoint_M`
  (params (ui_KOTH :type "/Game/Alex-d016946l/Alex_GameModes/UI_KOTH Object Reference") (BP_ControlPoint :type "/Game/Alex-d016946l/ControlPoint/BP_ControlPoint Object Reference"))
  ;[1 0.6431 0] Init
  (bind _output_get (set `self.Ui KOTH` ui_KOTH))
  (`/Game/Alex-d016946l/Alex_GameModes/UI_KOTH.Init_Texture` _output_get "/Game/Alex-d016946l/ControlPoint/Materials_and_textures/ControlPointYellow.ControlPointYellow")
  (set `self.ControlPoint_ref` BP_ControlPoint))

(event `Increasing score Team_A`
  ;[1 1 1] When the control point is captured, it will increase the score for the team
  (bind (_direction _team_a_progress _team_a_seconds_left) (`Timeline|Team A score` :!label _label)
    (:`Update`
      (`ProgressBar.SetPercent` (`/Game/Alex-d016946l/Alex_GameModes/UI_KOTH.ProgressBar_TeamA` (`self.Ui KOTH`)) _team_a_progress)
      (set `TextBlock.Text` (`KismetTextLibrary.Conv_DoubleToText` _team_a_seconds_left "HalfToEven") (`/Game/Alex-d016946l/Alex_GameModes/UI_KOTH.Text_TimeLeft_TeamA` (`self.Ui KOTH`))))
    (:`Finished`
      (bind _result (`/Engine/EditorBlueprintResources/StandardMacros.IncrementInt` (`self.RoundsWon_TeamA`))
        (:`  `
          (`/Game/Alex-d016946l/Alex_GameModes/UI_KOTH.Get_Texture` (`self.Ui KOTH`) (`self.Blue_Texture`) _result true)
          (`self.SetActorTickEnabled` (`self.ControlPoint_ref`) false)
          (message `/Game/Alex-d016946l/Interfaces/BPI_KOTH.I_RoundOver` (`GameplayStatics.GetGameMode`) "NewEnumerator1")
          (`self.Set score new time`))))))

(event `Stop Scoring Team_A`
  ;[1 1 1] When the control point is captured, it will increase the score for the team
  (goto _label :!via `Stop`))

(event `Stop Scoring Team_Both`
  ;[1 1 1] When the control point is captured, it will increase the score for the team
  (`|ExecutionSequence`
    (:`then_0`
      (goto _label :!via `Stop`))
    (:`then_1`
      (bind (_direction _team_b_progress _team_b_seconds_left) (`Timeline|Team B Score` :!via `Stop` :!label _label_2)
        (:`Update`
          (`ProgressBar.SetPercent` (`/Game/Alex-d016946l/Alex_GameModes/UI_KOTH.ProgressBar_TeamB` (`self.Ui KOTH`)) _team_b_progress)
          (set `TextBlock.Text` (`KismetTextLibrary.Conv_DoubleToText` _team_b_seconds_left "HalfToEven") (`/Game/Alex-d016946l/Alex_GameModes/UI_KOTH.Text_TimeLeft_TeamB` (`self.Ui KOTH`))))
        (:`Finished`
          (bind _result (`/Engine/EditorBlueprintResources/StandardMacros.IncrementInt` (`self.RoundsWon_TeamB`))
            (:`  `
              (`/Game/Alex-d016946l/Alex_GameModes/UI_KOTH.Get_Texture` (`self.Ui KOTH`) (`self.Red_Texture`) _result false)
              (`self.SetActorTickEnabled` (`self.ControlPoint_ref`) false)
              (message `/Game/Alex-d016946l/Interfaces/BPI_KOTH.I_RoundOver` (`GameplayStatics.GetGameMode`) "NewEnumerator2")
              (`self.Set score new time`))))))))

(event `Increasing score Team_B`
  ;[1 1 1] When the control point is captured, it will increase the score for the team
  (goto _label_2))

(event `Stop Scoring Team_B`
  ;[1 1 1] When the control point is captured, it will increase the score for the team
  (goto _label_2 :!via `Stop`))

(fn `Set score new time`
  (`TimelineComponent.SetNewTime` (`self.Team A score`) 0.0)
  (`TimelineComponent.SetNewTime` (`self.Team B Score`) 0.0))

(fn `UserConstructionScript`)
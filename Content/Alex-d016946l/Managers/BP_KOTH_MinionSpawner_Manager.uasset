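; BP_KOTH_MinionSpawner_Manager triggers periodic minion spawn waves across a set of referenced spawners, apparently for a King of the Hill mode.
; Initialization fires a wave immediately and starts a looping 30-second timer for further spawning.
; Each wave starts every spawner's own spawn timer, then clears it after a short delay, so spawning runs in brief bursts.
; A separate event clears the manager's looping timer.
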(event `Init_MinionSpawner_M`
  (`self.TellSpawner to spawn`)
  (bind _returnvalue (`KismetSystemLibrary.K2_SetTimerDelegate` (`|CreateDelegate` :!event `TellSpawner to spawn`) 30.0 true))
  (set `self.TimerHandle` _returnvalue))

(event `TellSpawner to spawn`
  (for _array_element (`self.MinionSpawners_ref`)
    (`/Game/Alex-d016946l/Minions/BP_MinionSpawner.Set_Timer_MinionSpawn` _array_element))
  (`KismetSystemLibrary.Delay` 1.1)
  (for _array_element_2 (`self.MinionSpawners_ref`)
    (`/Game/Alex-d016946l/Minions/BP_MinionSpawner.Clear_Handle_MinionSpawn` _array_element_2)))

(event `Clear MinionSpawner_M handle`
  (`KismetSystemLibrary.K2_ClearAndInvalidateTimerHandle` (`self.TimerHandle`)))

(fn `MinionSpawn_Timer`)

(fn `UserConstructionScript`)
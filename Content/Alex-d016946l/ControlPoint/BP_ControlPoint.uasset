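; BP_ControlPoint is a team control point actor that currently only reports which players are inside it.
; Init_ControlPoint stores the player controllers and both team rosters.
; Each Box begin overlap polls all overlapping third-person characters through an interface message and prints their ID, name, class and team.
; Logic to switch the decal between blue and red materials by team exists but is disconnected.
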(event `Init_ControlPoint`
  (params (GameplayControllers :type "Array of /Game/c013265l/Blueprints/PlayerControllers/PC_Game Object Reference") (TeamA_Players :type "Array of /Game/c013265l/Blueprints/PlayerControllers/PC_Game Object Reference") (TeamB_Players :type "Array of /Game/c013265l/Blueprints/PlayerControllers/PC_Game Object Reference"))
  (set `self.PlayerControllers` GameplayControllers)
  (set `self.Team A Players` TeamA_Players)
  (set `self.Team B Players` TeamB_Players))

(event `self.Box.OnComponentBeginOverlap`
  (params (OverlappedComponent :type "PrimitiveComponent Object Reference") (OtherActor :type "Actor Object Reference") (OtherComp :type "PrimitiveComponent Object Reference") (OtherBodyIndex :type Integer) (bFromSweep :type Boolean) (SweepResult :type "HitResult Structure (by ref)"))
  (for _array_element (`PrimitiveComponent.GetOverlappingActors` (`self.Box`) "/Game/ThirdPerson/Blueprints/BP_ThirdPersonCharacter.BP_ThirdPersonCharacter_C")
    (bind _playerdata (message `/Game/c013265l/Blueprints/Interfaces/BPI_Teams.I_GetPlayerData` _array_element))
    (bind (_playerid _playername _playerclass _teamid) (break `/Game/c013265l/Structs/S_PlayerData` _playerdata))
    (`KismetSystemLibrary.PrintString` (`KismetStringLibrary.Concat_StrStr` "Player ID: " (`KismetStringLibrary.Conv_IntToString` _playerid) "        PLAYER NAME: " (`KismetTextLibrary.Conv_TextToString` _playername) "      CLASS: " (`KismetSystemLibrary.GetClassDisplayName` _playerclass) "       " (`|GetEnumeratorNameAsString` _teamid)))))

(fn `UserConstructionScript`)
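; Zombie enemy that melees the player and reports its death to the game mode with the killer's team.
; AttackPlayer sphere-traces forward for pawns and, after a delay, damages the blackboard TargetActor rather than the traced hit.
; AnyDamage feeds Health, which destroys the zombie at zero.
; Health never writes its local result back to CharacterStats, so damage does not accumulate in this graph.
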(event `self.ReceiveAnyDamage`
  (params (Damage :type "Float (single-precision)") (DamageType :type "DamageType Object Reference") (InstigatedBy :type "Controller Object Reference") (DamageCauser :type "Actor Object Reference"))
  (`self.Health` Damage false InstigatedBy))

(event `Attack Player`
  (bind _returnvalue (`self.K2_GetActorLocation`))
  (bind (_outhit _returnvalue_2) (`KismetSystemLibrary.SphereTraceSingleForObjects` _returnvalue (+ _returnvalue (* (`KismetMathLibrary.GetForwardVector` (`self.K2_GetActorRotation`)) 250.0)) 80.0 (`|MakeArray` "ObjectTypeQuery3" :!type "EObjectTypeQuery Enum") true))
  (if _returnvalue_2
    (`KismetSystemLibrary.Delay` 3.0)
    (`self.Attack`)))

(fn `Attack`
  (bind _asbp_third_person_character (cast `/Game/ThirdPerson/Blueprints/BP_ThirdPersonCharacter` (`BlackboardComponent.GetValueAsObject` (`AIBlueprintHelperLibrary.GetBlackboard` (`self.GetController`)) "TargetActor")))
  (`/Game/ThirdPerson/Blueprints/BP_ThirdPersonCharacter.ModifyHealth` _asbp_third_person_character 5.0 false "")
  (`KismetSystemLibrary.PrintString` (`KismetStringLibrary.Conv_DoubleToString` (`.CurrentHealth_4_E7CB1D7448D4E0198F1304A316B5B9E5` (break `/Game/c013265l/Blueprints/StructsData/S_CharacterStats` (`/Game/ThirdPerson/Blueprints/BP_ThirdPersonCharacter.CharacterStats` _asbp_third_person_character))))))

(fn `Health`
  (params (`Health Modify` :type "Float (double-precision)") (IsHealing :type Boolean) (AttackerRef :type "Controller Object Reference"))
  (locals (L_CurrentHealth :type "Float (double-precision)"))
  (bind ((`MaxHealth_2_901ADD2C4C74E5308EC359A5539E7D95` _maxhealth) (`CurrentHealth_4_E7CB1D7448D4E0198F1304A316B5B9E5` _currenthealth)) (break `/Game/c013265l/Blueprints/StructsData/S_CharacterStats` (`self.CharacterStats`)))
  (bind _returnvalue (+ _currenthealth `Health Modify`))
  (if IsHealing
    (if (> _returnvalue _maxhealth)
      (set `local.L_CurrentHealth` _maxhealth)
      (else
        (set `local.L_CurrentHealth` _returnvalue)))
    (else
      (set `local.L_CurrentHealth` (- _currenthealth `Health Modify`))))
  (if (<= (`local.L_CurrentHealth`) 0.0)
    (bind _teamid (message `/Game/c013265l/Blueprints/Interfaces/BPI_Teams.I_GetTeam` AttackerRef))
    (message `/Game/BPI_Zombies.I_On Zombie Death` (`GameplayStatics.GetGameMode`) _teamid AttackerRef)
    (`self.K2_DestroyActor`)))

(fn `UserConstructionScript`)
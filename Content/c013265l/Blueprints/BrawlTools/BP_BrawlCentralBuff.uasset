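; Destructible central buff objective for Brawl mode that rewards the team that depletes its health with a damage modifier.
; On init it binds to GM_Brawl to receive and cache the controller list.
; Damage lowers Health; at zero or below, it writes DamageModifier into the character stats of pawns on the DamageCauser's team through interface messages.
; It neither destroys itself nor guards against repeat triggers.
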(event `/Game/c013265l/Blueprints/Interfaces/BPI_Brawl.I_InitCentralBuff`
  (add `/Game/c013265l/Blueprints/GameModes/GM_Brawl.CommunicateControllerList` (cast `/Game/c013265l/Blueprints/GameModes/GM_Brawl` (`GameplayStatics.GetGameMode`) :!pure true) (delegate `GetControllers`)))

(event `GetControllers`
  (params (ControllerList :type "Array of /Game/c013265l/Blueprints/PlayerControllers/PC_Game Object Reference (by ref)"))
  (set `self.Controller List` ControllerList))

(event `self.ReceiveAnyDamage`
  (params (Damage :type "Float (single-precision)") (DamageType :type "DamageType Object Reference") (InstigatedBy :type "Controller Object Reference") (DamageCauser :type "Actor Object Reference"))
  (bind _output_get (set `self.Health` (- (`self.Health`) Damage)))
  (if (<= _output_get 0.0)
    (bind _teamid (message `/Game/c013265l/Blueprints/Interfaces/BPI_Teams.I_GetTeam` DamageCauser))
    (for _array_element (`self.Controller List`)
      (bind _teamid_2 (message `/Game/c013265l/Blueprints/Interfaces/BPI_Teams.I_GetTeam` _array_element))
      (if (`|EnumEquality` _teamid_2 _teamid)
        (bind _returnvalue (`Controller.K2_GetPawn` _array_element))
        (bind _characterstats (message `/Game/c013265l/Blueprints/Interfaces/BPI_PawnCommunication.I_GetCharacterStats` _returnvalue))
        (bind _structout (setmembers `/Game/c013265l/Blueprints/StructsData/S_CharacterStats` :`StructRef` _characterstats :`DamageModifier` (`self.DamageModifier`)))
        (message `/Game/c013265l/Blueprints/Interfaces/BPI_PawnCommunication.I_SetCharacterStats` _returnvalue _structout)))))

(fn `UserConstructionScript`)
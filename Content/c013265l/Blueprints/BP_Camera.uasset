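; Shared multiplayer camera that frames up to four registered characters, dropping them on death.
; Once adjusting starts, each tick gathers living positions, targeting the midpoint for two or a minimum-area rectangle's center for three or four.
; It interpolates toward that target and sets clamped spring-arm length from player spread.
; Zero- and one-player cases set targets without moving the camera; the pairwise-distance logic and NewCameraPosition are unused leftovers.
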(event `/Game/c013265l/Blueprints/Interfaces/BPI_Camera.I_SetupCharacterRefs`
  (params (NewCharacterRef :type "Pawn Object Reference"))
  (`/Engine/EditorBlueprintResources/StandardMacros.IsValid` NewCharacterRef
    (:`Is Valid`
      (`KismetArrayLibrary.Array_AddUnique` (`self.Characters`) NewCharacterRef))))

(event `/Game/c013265l/Blueprints/Interfaces/BPI_RoundManagement.I_PlayerDeath`
  (params (TeamID :type "/Game/c013265l/Gameplay/Enum_Teams Enum" :default "NewEnumerator0") (DeadPawn :type "Pawn Object Reference"))
  (`KismetArrayLibrary.Array_RemoveItem` (`self.Characters`) DeadPawn))

(event `/Game/c013265l/Blueprints/Interfaces/BPI_Camera.I_StartAdjusting`
  (bind _output_get (set `self.OldCameraPosition` (`self.K2_GetActorLocation`)))
  (bind _output_get_2 (set `self.NewCameraPosiion` _output_get))
  (set `self.StartingLocation` _output_get_2)
  (set `self.CanAdjust` true))

(event `self.ReceiveTick`
  (params (DeltaSeconds :type "Float (single-precision)"))
  (bind _playerlocations (`self.PlayerLocations`))
  (bind _playerlocations_2 (`self.PlayerLocations`))
  (if (`self.CanAdjust`)
    (`KismetArrayLibrary.Array_Clear` (`self.PlayerLocations`))
    (`KismetArrayLibrary.Array_Clear` (`self.Distances`))
    (for _array_element (`self.Characters`)
      (`/Engine/EditorBlueprintResources/StandardMacros.IsValid` _array_element
        (:`Is Valid`
          (`KismetArrayLibrary.Array_AddUnique` (`self.PlayerLocations`) (`self.K2_GetActorLocation` _array_element)))))
    (switch `int` (`KismetArrayLibrary.Array_Length` (`self.PlayerLocations`))
      (:`0`
        (set `self.NewDistance` 1200.0)
        (set `self.NewCameraPosiion` (`self.StartingLocation`)))
      (:`1`
        (set `self.NewDistance` 1200.0)
        (set `self.NewCameraPosiion` (`|GetArrayItem` (`self.PlayerLocations`))))
      (:`2`
        (set `self.NewDistance` (`KismetMathLibrary.Abs` (`KismetMathLibrary.VSize` (- (`|GetArrayItem` _playerlocations_2) (`|GetArrayItem` _playerlocations_2 1)))))
        (set `self.NewCameraPosiion` (/ (+ (`|GetArrayItem` _playerlocations) (`|GetArrayItem` _playerlocations 1)) 2.0))
        (bind _output_get (set `self.Focus` (`KismetMathLibrary.VInterpTo` (`self.OldCameraPosition`) (`self.NewCameraPosiion`) (`GameplayStatics.GetWorldDeltaSeconds`) (`self.InterpSpeed`)) :!label _label))
        (`self.K2_SetActorLocation` _output_get)
        (set `self.OldCameraPosition` (`self.K2_GetActorLocation`))
        (set `SpringArmComponent.TargetArmLength` (`KismetMathLibrary.FClamp` (`self.NewDistance`) 1600.0 3000.0) (`self.SpringArm`))
        (set `self.InterpSpeed` (/ (`KismetMathLibrary.VSize` (`self.Focus`)) 500.0)))
      (:`3`
        (bind (_outrectcenter _outrectrotation _outrectlengthx _outrectlengthy) (`KismetMathLibrary.MinAreaRectangle` (`self.PlayerLocations`) (`self.K2_GetActorLocation`) :!label _label_2))
        (set `self.NewDistance` (`KismetMathLibrary.Sqrt` (+ (`KismetMathLibrary.Square` _outrectlengthx) (`KismetMathLibrary.Square` _outrectlengthy))))
        (set `self.NewCameraPosiion` _outrectcenter)
        (goto _label))
      (:`4`
        (goto _label_2)))))

(fn `NewCameraPosition`
  (bind _index (`self.Index`))
  (`KismetSystemLibrary.PrintString` (`KismetStringLibrary.Conv_IntToString` _index) true true (struct :`R` 0.016312 :`G` 1.0 :`A` 1.0))
  (switch `int` _index
    (:`0`
      (set `self.NewCameraPosiion` (/ (+ (`self.K2_GetActorLocation` (`|GetArrayItem` (`self.Characters`))) (`self.K2_GetActorLocation` (`|GetArrayItem` (`self.Characters`) 1))) 2.0) :!label _label))
    (:`1`
      (goto _label))
    (:`2`
      (set `self.NewCameraPosiion` (/ (+ (`self.K2_GetActorLocation` (`|GetArrayItem` (`self.Characters`))) (`self.K2_GetActorLocation` (`|GetArrayItem` (`self.Characters`) 2))) 2.0)))
    (:`3`
      (set `self.NewCameraPosiion` (/ (+ (`self.K2_GetActorLocation` (`|GetArrayItem` (`self.Characters`))) (`self.K2_GetActorLocation` (`|GetArrayItem` (`self.Characters`) 3))) 2.0)))
    (:`6`
      (set `self.NewCameraPosiion` (/ (+ (`self.K2_GetActorLocation` (`|GetArrayItem` (`self.Characters`) 1)) (`self.K2_GetActorLocation` (`|GetArrayItem` (`self.Characters`) 2))) 2.0)))
    (:`7`
      (set `self.NewCameraPosiion` (/ (+ (`self.K2_GetActorLocation` (`|GetArrayItem` (`self.Characters`) 1)) (`self.K2_GetActorLocation` (`|GetArrayItem` (`self.Characters`) 3))) 2.0)))
    (:`11`
      (set `self.NewCameraPosiion` (/ (+ (`self.K2_GetActorLocation` (`|GetArrayItem` (`self.Characters`) 2)) (`self.K2_GetActorLocation` (`|GetArrayItem` (`self.Characters`) 3))) 2.0)))))

(fn `UserConstructionScript`)
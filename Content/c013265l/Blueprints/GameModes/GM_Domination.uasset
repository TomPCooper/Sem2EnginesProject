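; Game mode for local multiplayer two-team Domination, a tug-of-war along staged control points that starts mid-chain.
; Init creates up to four players from GameInstance data, spawns pawns at team starts on a map camera, then sets up UI, points and pickups.
; Captures update scores and shift the active stage; deaths trigger timed respawns.
; GameState drives match phases; timeout, passing either chain end or collecting all pickups returns to the menu.
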(event `Init`
  (`self.SetUpControllerGI`)
  (`self.SpawnCharacters`)
  (`self.BindToGameState`)
  (`/Game/c013265l/Blueprints/PlayerControllers/PC_Game.Init` (`self.GamePlayControllers`))
  (`self.SetupUI`)
  (`self.SetupControlPoints`)
  (`self.InitPickups`)
  (`KismetSystemLibrary.Delay` 2.0)
  (`/Game/c013265l/Blueprints/GameStates/GS_GameStateBase.UpdateState` (`self.GS_GameState`) "NewEnumerator1"))

(event `BindToGameState`
  (bind _output_get (set `self.GS_GameState` (cast `/Game/c013265l/Blueprints/GameStates/GS_GameStateBase` (`GameplayStatics.GetGameState`) :!pure true)))
  (add `/Game/c013265l/Blueprints/GameStates/GS_GameStateBase.GameStateChanged` _output_get (`|CreateDelegate` :!event `GameStateChanged`)))

(event `self.ReceiveBeginPlay`
  (set `self.GameInstance` (cast `/Game/c013265l/Blueprints/GameInstances/GameInstance` (`GameplayStatics.GetGameInstance`) :!pure true))
  (bind _returnvalue (`GameplayStatics.GetActorOfClass` "/Game/c013265l/Blueprints/BP_Camera.BP_Camera_C"))
  (set `self.MapCamera` _returnvalue)
  (`self.Init`))

(event `EndGame`
  (`KismetSystemLibrary.Delay` 3.0)
  (`/Game/c013265l/Blueprints/FucntionLibraries/BPL_GamePlay.RemoveAllPlayers`)
  (`GameplayStatics.OpenLevel` "Menu_Main"))

(event `/Game/c013265l/Blueprints/Interfaces/BPI_RoundManagement.I_PlayerDeath`
  (params (TeamID :type "/Game/c013265l/Gameplay/Enum_Teams Enum" :default "NewEnumerator0") (DeadPawn :type "Pawn Object Reference"))
  ;[0 0 0] On Player death - c013265;l
  (message `/Game/c013265l/Blueprints/Interfaces/BPI_Respawn.I_StartRespawnTimer` (`Pawn.GetController` DeadPawn) 12.0)
  (switch `/Game/c013265l/Gameplay/Enum_Teams` TeamID
    (:`NewEnumerator1`
      (`/Engine/EditorBlueprintResources/StandardMacros.IncrementInt` (`self.TeamBKills`)))
    (:`NewEnumerator2`
      (`/Engine/EditorBlueprintResources/StandardMacros.IncrementInt` (`self.TeamAKills`)))))

(event `/Game/c013265l/Blueprints/Interfaces/BPI_Respawn.I_RespawnPlayer`
  (params (Controller :type "/Game/c013265l/Blueprints/PlayerControllers/PC_Game Object Reference") (TeamID :type "/Game/c013265l/Gameplay/Enum_Teams Enum" :default "NewEnumerator0"))
  (`self.RespawnCharacter` TeamID null Controller))

(event `GameStateChanged`
  (params (CurrentGameState :type "/Game/c013265l/Blueprints/Enumerators/E_GameState Enum" :default "NewEnumerator0"))
  (switch `/Game/c013265l/Blueprints/Enumerators/E_GameState` CurrentGameState
    (:`NewEnumerator1`
      (`KismetSystemLibrary.PrintString` "Pre Game")
      (`KismetSystemLibrary.Delay` 3.0)
      (`/Game/c013265l/Blueprints/GameStates/GS_GameStateBase.UpdateState` (`self.GS_GameState`) "NewEnumerator2"))
    (:`NewEnumerator2`
      (`KismetSystemLibrary.PrintString` "InGame")
      (`KismetSystemLibrary.K2_SetTimerDelegate` (`|CreateDelegate` :!event `TimeUp`) 300.0))
    (:`NewEnumerator3`
      (`KismetSystemLibrary.PrintString` "EndingGame")
      (`self.EndGame`))))

(event `InitPickups`
  (bind _outactors (`GameplayStatics.GetAllActorsOfClass` "/Game/c013265l/Blueprints/PickUps/BP_Pickup.BP_Pickup_C"))
  (bind _output_get (set `self.PickUpActorsRemaining` _outactors))
  (add `/Game/c013265l/Blueprints/PickUps/BP_Pickup.PickupCollected` _output_get (`|CreateDelegate` :!event `PickupCollected`)))

(event `TimeUp`
  (set `self.HasTimeRanOut` true)
  (`self.CanEndGame`))

(event `self.K2_PostLogin`
  (params (NewPlayer :type "PlayerController Object Reference"))
  (bind _aspc_game (cast `/Game/c013265l/Blueprints/PlayerControllers/PC_Game` NewPlayer))
  (`KismetArrayLibrary.Array_Add` (`self.GamePlayControllers`) _aspc_game))

(event `self.K2_OnLogout`
  (params (ExitingController :type "Controller Object Reference"))
  (bind _aspc_game (cast `/Game/c013265l/Blueprints/PlayerControllers/PC_Game` ExitingController))
  (`KismetArrayLibrary.Array_RemoveItem` (`self.GamePlayControllers`) _aspc_game)
  (`KismetArrayLibrary.Array_RemoveItem` (`self.TeamA_Players`) _aspc_game)
  (`KismetArrayLibrary.Array_RemoveItem` (`self.TeamB_Players`) _aspc_game))

(event `PickupCollected`
  (params (PickupActorRef :type "/Game/c013265l/Blueprints/PickUps/BP_Pickup Object Reference"))
  (bind _pickupactorsremaining (`self.PickUpActorsRemaining`))
  (`KismetArrayLibrary.Array_RemoveItem` _pickupactorsremaining PickupActorRef)
  (if (== (`KismetArrayLibrary.Array_Length` _pickupactorsremaining) 0)
    (set `self.AllPointsCaptured` true)
    (`self.CanEndGame`)))

(event `/Game/c013265l/Blueprints/Interfaces/BPI_Domination.I_AddPoints`
  (params (TeamID :type "/Game/c013265l/Gameplay/Enum_Teams Enum" :default "NewEnumerator0")))

(event `/Game/c013265l/Blueprints/Interfaces/BPI_Domination.I_AdvanceRound`
  (params (TeamWon :type "/Game/c013265l/Gameplay/Enum_Teams Enum" :default "NewEnumerator0"))
  (bind _currentstage (`self.CurrentStage`))
  (switch `/Game/c013265l/Gameplay/Enum_Teams` TeamWon
    (:`NewEnumerator1`
      (`/Engine/EditorBlueprintResources/StandardMacros.IncrementInt` _currentstage
        (:`  `
          (bind _result (`/Engine/EditorBlueprintResources/StandardMacros.IncrementInt` (`self.TeamAPoints`))
            (:`  `
              (`TextBlock.SetText` (`/Game/c013265l/UI/UI_Domination.TextAScore` (`self.DominationUI`)) (`KismetTextLibrary.Conv_IntToText` _result))
              (if (> (`self.CurrentStage`) 6)
                (set `self.AllPointsCaptured` true)
                (`self.CanEndGame`)
                (else
                  (message `/Game/c013265l/Blueprints/Interfaces/BPI_Domination.I_SetActiveControlPoint` (`|GetArrayItem` (`self.ControlPoints`) (`self.CurrentStage`)) true)
                  (`KismetSystemLibrary.PrintString` (`KismetStringLibrary.Concat_StrStr` "next control point = " (`KismetStringLibrary.Conv_IntToString` (`self.CurrentStage`))) :!label _label))))))))
    (:`NewEnumerator2`
      (`/Engine/EditorBlueprintResources/StandardMacros.DecrementInt` _currentstage
        (:`  `
          (bind _result_2 (`/Engine/EditorBlueprintResources/StandardMacros.IncrementInt` (`self.TeamBPoints`))
            (:`  `
              (`TextBlock.SetText` (`/Game/c013265l/UI/UI_Domination.TextBScore` (`self.DominationUI`)) (`KismetTextLibrary.Conv_IntToText` _result_2))
              (if (< (`self.CurrentStage`) 1)
                (set `self.AllPointsCaptured` true)
                (`self.CanEndGame`)
                (else
                  (message `/Game/c013265l/Blueprints/Interfaces/BPI_Domination.I_SetActiveControlPoint` (`|GetArrayItem` (`self.ControlPoints`) (`self.CurrentStage`)) true)
                  (goto _label))))))))))

(fn `AddToTeamLists`
  (params (GameplayController :type "/Game/c013265l/Blueprints/PlayerControllers/PC_Game Object Reference"))
  (bind _teamid (message `/Game/c013265l/Blueprints/Interfaces/BPI_Teams.I_GetTeam` GameplayController))
  (switch `/Game/c013265l/Gameplay/Enum_Teams` _teamid
    (:`NewEnumerator1`
      (`KismetArrayLibrary.Array_Add` (`self.TeamA_Players`) GameplayController))
    (:`NewEnumerator2`
      (`KismetArrayLibrary.Array_Add` (`self.TeamB_Players`) GameplayController))))

(fn `CanEndGame`
  (if (or (`self.HasTimeRanOut`) (`self.HaveAllPlayersDied`) (`self.AllPointsCaptured`))
    (`/Game/c013265l/Blueprints/GameStates/GS_GameStateBase.UpdateState` (`self.GS_GameState`) "NewEnumerator3")))

(fn `ChoosePlayerStart`
  (params (Player :type "Controller Object Reference"))
  (returns (ReturnValue :type "Actor Object Reference"))
  (return null))

(fn `RespawnCharacter`
  (params (TeamID :type "/Game/c013265l/Gameplay/Enum_Teams Enum" :default "NewEnumerator0") (CharacterToRespawn :type "Pawn Object Reference") (Controller :type "/Game/c013265l/Blueprints/PlayerControllers/PC_Game Object Reference"))
  (bind _playerdata (message `/Game/c013265l/Blueprints/Interfaces/BPI_Teams.I_GetPlayerData` Controller))
  (bind _returnvalue (`|SpawnActorFromClass` (`.PlayerClass_13_AB63BDD64175B900ED43C68475968EA3` (break `/Game/c013265l/Structs/S_PlayerData` _playerdata)) (`self.GetTransform` (`self.SelectPlayerStart` TeamID)) "AdjustIfPossibleButAlwaysSpawn" "OverrideRootScale" null null))
  (`Controller.Possess` Controller _returnvalue))

(fn `SelectPlayerStart`
  (params (TeamID :type "/Game/c013265l/Gameplay/Enum_Teams Enum" :default "NewEnumerator0"))
  (returns (StartActor :type "/Game/c013265l/Gameplay/BP_TeamPlayerStart Object Reference"))
  (locals (L_SpawnPointActors :type "Array of /Game/c013265l/Gameplay/BP_TeamPlayerStart Object Reference"))
  (bind _outactors (`GameplayStatics.GetAllActorsOfClass` "/Game/c013265l/Gameplay/BP_TeamPlayerStart.BP_TeamPlayerStart_C"))
  (for _array_element _outactors
    (bind _teamid (message `/Game/c013265l/Blueprints/Interfaces/BPI_Teams.I_GetTeam` _array_element))
    (if (`|EnumEquality` _teamid TeamID)
      (`KismetArrayLibrary.Array_Add` (`local.L_SpawnPointActors`) _array_element)))
  (if (!= (`KismetArrayLibrary.Array_Length` (`local.L_SpawnPointActors`)) 0)
    (return (`KismetArrayLibrary.Array_Random` (`local.L_SpawnPointActors`)))
    (else
      (bind _returnvalue (`GameplayStatics.GetActorOfClass` "/Game/c013265l/Gameplay/BP_TeamPlayerStart.BP_TeamPlayerStart_C"))
      (return _returnvalue))))

(fn `SetUpController`
  (params (PlayerCount :type Integer))
  (`GameplayStatics.RemovePlayer` (`GameplayStatics.GetPlayerController` 0) true)
  (for _index (range PlayerCount)
    (bind _returnvalue (`GameplayStatics.CreatePlayer` _index))
    (`/Engine/EditorBlueprintResources/StandardMacros.FlipFlop`
      (:`A`
        (message `/Game/c013265l/Blueprints/Interfaces/BPI_Teams.I_SetTeam` _returnvalue "NewEnumerator1"))
      (:`B`
        (message `/Game/c013265l/Blueprints/Interfaces/BPI_Teams.I_SetTeam` _returnvalue "NewEnumerator2")))
    (`self.AddToTeamLists` (cast `/Game/c013265l/Blueprints/PlayerControllers/PC_Game` _returnvalue :!pure true))))

(fn `SetUpControllerGI`
  (bind _gameinstance (`self.GameInstance`))
  (`GameplayStatics.RemovePlayer` (`GameplayStatics.GetPlayerController` 0))
  (for _index (range 4)
    (bind _returnvalue (select `int` _index :`0` (`/Game/c013265l/Blueprints/GameInstances/GameInstance.Player0_data` _gameinstance) :`1` (`/Game/c013265l/Blueprints/GameInstances/GameInstance.Player1_data` _gameinstance) :`2` (`/Game/c013265l/Blueprints/GameInstances/GameInstance.Player2_data` _gameinstance) :`3` (`/Game/c013265l/Blueprints/GameInstances/GameInstance.Player3_data` _gameinstance)))
    (bind ((`PlayerID_2_B9C8EF28415CAA77CC6887A2B3E5FC49` _playerid) (`PlayerClass_13_AB63BDD64175B900ED43C68475968EA3` _playerclass) (`IsActive_19_07E58887427E7C144A22AE87F1E11D74` _isactive)) (break `/Game/c013265l/Structs/S_PlayerData` _returnvalue))
    (if _isactive
      (bind _returnvalue_2 (`GameplayStatics.CreatePlayer` _playerid))
      (message `/Game/c013265l/Blueprints/Interfaces/BPI_Teams.I_SetPlayerData` _returnvalue_2 _returnvalue)
      (`self.AddToTeamLists` (cast `/Game/c013265l/Blueprints/PlayerControllers/PC_Game` _returnvalue_2 :!pure true)))))

(fn `SetupControlPoints`
  (bind _output (`|GetArrayItem` (`self.ControlPoints`) 3))
  (bind _outactors (`GameplayStatics.GetAllActorsOfClass` "/Game/c013265l/DominationTools/BP_DominationControlPoint.BP_DominationControlPoint_C"))
  (for _array_element _outactors
    (`KismetArrayLibrary.Array_Set` (`self.ControlPoints`) (`/Game/c013265l/DominationTools/BP_DominationControlPoint.Stage` _array_element) _array_element true)
    (message `/Game/c013265l/Blueprints/Interfaces/BPI_Domination.I_SetUI` _array_element (`self.DominationUI`)))
  (set `self.ActiveControlPoint` _output)
  (message `/Game/c013265l/Blueprints/Interfaces/BPI_Domination.I_SetActiveControlPoint` _output true))

(fn `SetupUI`
  (bind _returnvalue (`|CreateWidget` "/Game/c013265l/UI/UI_Domination.UI_Domination_C"))
  (bind _output_get (set `self.DominationUI` _returnvalue))
  (`UserWidget.AddToViewport` _output_get 0))

(fn `SpawnCharacters`
  (for _array_element (`self.GamePlayControllers`)
    (bind _playerdata (message `/Game/c013265l/Blueprints/Interfaces/BPI_Teams.I_GetPlayerData` _array_element))
    (bind ((`PlayerClass_13_AB63BDD64175B900ED43C68475968EA3` _playerclass) (`TeamID_16_C95AF1994DF53F697565858AC86BB26E` _teamid)) (break `/Game/c013265l/Structs/S_PlayerData` _playerdata))
    (bind _returnvalue (`|SpawnActorFromClass` _playerclass (`self.GetTransform` (`self.SelectPlayerStart` _teamid)) "AdjustIfPossibleButAlwaysSpawn" "OverrideRootScale" null null))
    (bind _aspawn (cast `Pawn` _returnvalue :!pure true))
    (`Controller.Possess` _array_element _aspawn)
    (message `/Game/c013265l/Blueprints/Interfaces/BPI_PawnCommunication.I_SetPawnTeam` _aspawn _teamid)
    (`PlayerController.SetViewTargetWithBlend` _array_element (`self.MapCamera`) 0.0 "VTBlend_Linear" 0.0 false)))

(fn `UserConstructionScript`)
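; GM_Menu is the main menu game mode that shows the menu and launches matches.
; On BeginPlay it creates UI_MainMenu, switches to UI-only input with a visible cursor and binds an event to the widget's start-game dispatcher.
; StartGame stores four players' data, level name and game mode alias in the GameInstance, then opens the level with that game mode alias and a hardcoded four-player count in the URL options.
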(event `self.ReceiveBeginPlay`
  (set `self.GameInstance` (cast `/Game/c013265l/Blueprints/GameInstances/GameInstance` (`GameplayStatics.GetGameInstance`) :!pure true))
  (`self.Init`))

(event `Init`
  (bind _returnvalue (`GameplayStatics.GetPlayerController` 0))
  (bind _returnvalue_2 (`|CreateWidget` "/Game/Demo/UI/UI_MainMenu.UI_MainMenu_C"))
  (bind _output_get (set `self.MainMenuWidget` _returnvalue_2))
  (`UserWidget.AddToViewport` _output_get 0)
  (`WidgetBlueprintLibrary.SetInputMode_UIOnlyEx` _returnvalue _output_get)
  (set `PlayerController.bShowMouseCursor` true _returnvalue)
  (add `/Game/Demo/UI/UI_MainMenu.StartGame` (`self.MainMenuWidget`) (`|CreateDelegate` :!event `StartGame`)))

(fn `StartGame`
  (params (Player0 :type "/Game/c013265l/Structs/S_PlayerData Structure") (Player1 :type "/Game/c013265l/Structs/S_PlayerData Structure") (Player2 :type "/Game/c013265l/Structs/S_PlayerData Structure") (Player3 :type "/Game/c013265l/Structs/S_PlayerData Structure") (LevelName :type Name) (GameModeAlias :type String))
  (`|ExecutionSequence`
    (:`then_0`
      (set `/Game/c013265l/Blueprints/GameInstances/GameInstance.Player0_data` (`local.Player0`) (`self.GameInstance`))
      (set `/Game/c013265l/Blueprints/GameInstances/GameInstance.Player1_data` (`local.Player1`) (`self.GameInstance`))
      (set `/Game/c013265l/Blueprints/GameInstances/GameInstance.Player2_data` (`local.Player2`) (`self.GameInstance`))
      (set `/Game/c013265l/Blueprints/GameInstances/GameInstance.Player3_data` (`local.Player3`) (`self.GameInstance`))
      (set `/Game/c013265l/Blueprints/GameInstances/GameInstance.LevelName` (`local.LevelName`) (`self.GameInstance`))
      (set `/Game/c013265l/Blueprints/GameInstances/GameInstance.GameModeAlias` (`local.GameModeAlias`) (`self.GameInstance`)))
    (:`then_1`
      (`WidgetBlueprintLibrary.SetInputMode_GameOnly` (`GameplayStatics.GetPlayerController` 0))
      (`GameplayStatics.OpenLevel` (`local.LevelName`) true (`KismetStringLibrary.Concat_StrStr` "Game=" (`local.GameModeAlias`) "?playerCount=" "4")))))

(fn `UserConstructionScript`)
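; PC_Game is the in-game player controller that holds the player's team ID and provides a shortcut back to the main menu.
; BeginPlay sets game-only input and hides the cursor, while pressing M removes all players and opens Menu_Main.
; Interface calls set and return TeamID.
; The volume damage event compares TeamID with the owning team but takes no action on the result.
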(event `self.ReceiveBeginPlay`
  (`WidgetBlueprintLibrary.SetInputMode_GameOnly` (`GameplayStatics.GetPlayerController` 0))
  (set `self.bShowMouseCursor` false))

(event `Key|M`
  (params (Key :type "Key Structure"))
  (:`Pressed`
    (`/Game/c013265l/Blueprints/FucntionLibraries/BPL_GamePlay.RemoveAllPlayers`)
    (`GameplayStatics.OpenLevel` "Menu_Main")))

(event `self.I_SetTeam`
  (params (TeamID :type "/Game/c013265l/Gameplay/Enum_Teams Enum" :default "NewEnumerator0"))
  (set `self.Team ID` TeamID))

(event `/Game/c013265l/Blueprints/Interfaces/BPI_Damage.I_VolumeDamage`
  (params (OwningTeam :type "/Game/c013265l/Gameplay/Enum_Teams Enum" :default "NewEnumerator0"))
  (bind _teamid (`self.I_GetTeam`))
  (if (`|EnumEquality` _teamid OwningTeam)
    _))

(fn `I_GetTeam`
  (returns (TeamID :type "/Game/c013265l/Gameplay/Enum_Teams Enum"))
  (return (`self.Team ID`)))

(fn `UserConstructionScript`)
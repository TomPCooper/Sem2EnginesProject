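; GameInstance Blueprint that stores round or match win counts for two teams, Team A and Team B.
; AddWin increments the counter for the given team, and ResetWins sets both back to zero.
; GetWins returns a team's count by team ID, with No Team returning zero.
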(event `ResetWins`
  (set `self.TeamA_Wins` 0)
  (set `self.TeamB_Wins` 0))

(event `AddWin`
  (params (TeamID :type "/Game/c013265l/Gameplay/Enum_Teams Enum" :default "NewEnumerator0"))
  (switch `/Game/c013265l/Gameplay/Enum_Teams` TeamID
    (:`NewEnumerator1`
      (`/Engine/EditorBlueprintResources/StandardMacros.IncrementInt` (`self.TeamA_Wins`)))
    (:`NewEnumerator2`
      (`/Engine/EditorBlueprintResources/StandardMacros.IncrementInt` (`self.TeamB_Wins`)))))

(fn `GetWins`
  (params (TeamID :type "/Game/c013265l/Gameplay/Enum_Teams Enum" :default "NewEnumerator0"))
  (returns (Wins :type Integer))
  (switch `/Game/c013265l/Gameplay/Enum_Teams` TeamID
    (:`NewEnumerator0`
      (return 0))
    (:`NewEnumerator1`
      (return (`self.TeamA_Wins`)))
    (:`NewEnumerator2`
      (return (`self.TeamB_Wins`)))))
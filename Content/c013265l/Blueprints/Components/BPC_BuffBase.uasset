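; BPC_BuffBase is a base component for timed buffs applied to a character.
; Starting the buff sets a duration timer and, only once, caches the owner and its character stats, then calls StartBuffEffect with the modifier.
; On expiry it calls EndBuffEffect, tells the owner to remove the buff type via interface, and destroys itself.
; Both effect events are empty, left for child buffs to override.
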(event `/Game/c013265l/Blueprints/Interfaces/BPI_Pickups.I_StartBuffTimer`
  (params (BuffDuration :type "Float (double-precision)") (BuffOwner :type "Pawn Object Reference"))
  ;[0 0 0] c013265l Start Buff
  (`|ExecutionSequence`
    (:`then_0`
      (`KismetSystemLibrary.K2_SetTimerDelegate` (delegate `DestroyBuff`) BuffDuration))
    (:`then_1`
      (`/Engine/EditorBlueprintResources/StandardMacros.DoOnce` false
        (:`Completed`
          (bind _output_get (set `self.Buff Owner` BuffOwner))
          (bind _characterstats (message `/Game/c013265l/Blueprints/Interfaces/BPI_PawnCommunication.I_GetCharacterStats` _output_get))
          (set `self.Character Stats` _characterstats)
          (`self.StartBuffEffect` (`self.Modifier`)))))))

(event `DestroyBuff`
  ;[0 0 0] c013265l Start Buff
  (`self.EndBuffEffect`)
  (message `/Game/c013265l/Blueprints/Interfaces/BPI_Pickups.I_RemoveBuff` (stale `/Game/c013265l/Blueprints/Interfaces/BPI_Pickups.I_StartBuffTimer` BuffOwner) (`self.BuffType`))
  (`self.K2_DestroyComponent`))

(event `StartBuffEffect`
  (params (Modifier :type "Float (double-precision)"))
  ;[0 0 0] Events to Override
)

(event `EndBuffEffect`
  ;[0 0 0] Events to Override
)
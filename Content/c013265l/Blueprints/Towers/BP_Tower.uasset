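; BP_Tower is a team-owned defensive tower that damages one enemy at a time within its AttackRange.
; The first overlapping non-team actor implementing BPI_Damage passes a DoOnce lock, becomes CurrentTarget and starts a looping timer.
; StartFiring applies standard damage to that target.
; When the target leaves, a breakable loop picks another overlapping enemy character, but its completion clears the timer and target and resets the lock.
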(event `self.AttackRange.OnComponentBeginOverlap`
  (params (OverlappedComponent :type "PrimitiveComponent Object Reference") (OtherActor :type "Actor Object Reference") (OtherComp :type "PrimitiveComponent Object Reference") (OtherBodyIndex :type Integer) (bFromSweep :type Boolean) (SweepResult :type "HitResult Structure (by ref)"))
  (bind _teamid (message `/Game/c013265l/Blueprints/Interfaces/BPI_Teams.I_GetTeam` OtherActor))
  (if (`|EnumEquality` _teamid (`self.OwningTeam`))
    _
    (elif (`KismetSystemLibrary.DoesImplementInterface` OtherActor "/Game/c013265l/Blueprints/Interfaces/BPI_Damage.BPI_Damage_C")
      (`/Engine/EditorBlueprintResources/StandardMacros.DoOnce` false :!label _label
        (:`Completed`
          (set `self.CurrentTarget` OtherActor)
          (bind _returnvalue (`KismetSystemLibrary.K2_SetTimerDelegate` (`|CreateDelegate` :!event `StartFiring`) 2.0 true))
          (set `self.FireHandle` _returnvalue))))))

(event `ResetFiring`
  (goto _label :!via `Reset`))

(event `StartFiring`
  (`GameplayStatics.ApplyDamage` (`self.CurrentTarget`) 10.0 null null "/Game/c013265l/Blueprints/DamageTypes/BP_StandardDamage.BP_StandardDamage_C"))

(event `self.AttackRange.OnComponentEndOverlap`
  (params (OverlappedComponent :type "PrimitiveComponent Object Reference") (OtherActor :type "Actor Object Reference") (OtherComp :type "PrimitiveComponent Object Reference") (OtherBodyIndex :type Integer))
  (if (== OtherActor (`self.CurrentTarget`))
    (for _array_element (`PrimitiveComponent.GetOverlappingActors` (`self.AttackRange`) "/Game/ThirdPerson/Blueprints/BP_ThirdPersonCharacter.BP_ThirdPersonCharacter_C") :!label _label_2
      (bind _teamid (message `/Game/c013265l/Blueprints/Interfaces/BPI_Teams.I_GetTeam` _array_element))
      (if (not (`|EnumEquality` _teamid (`self.OwningTeam`)))
        (set `self.CurrentTarget` _array_element)
        (`self.StopSearching`)))
    (`KismetSystemLibrary.K2_ClearAndInvalidateTimerHandle` (`self.FireHandle`))
    (set `self.CurrentTarget` null)
    (`self.ResetFiring`)))

(event `StopSearching`
  (goto _label_2 :!via `Break`))

(fn `UserConstructionScript`)
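; BP_Pickup is a team-owned pickup that is destroyed when an actor without the Ignore tag overlaps its sphere.
; If that actor's team differs, it first notifies the game mode once through an interface message carrying the pickup's TeamID.
; TeamID is set through the ISpawnPickup interface event, and sphere query collision turns on shortly after BeginPlay.
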(event `self.Sphere1.OnComponentBeginOverlap`
  (params (OverlappedComponent :type "PrimitiveComponent Object Reference") (OtherActor :type "Actor Object Reference") (OtherComp :type "PrimitiveComponent Object Reference") (OtherBodyIndex :type Integer) (bFromSweep :type Boolean) (SweepResult :type "HitResult Structure (by ref)"))
  ;[1 0.8557 0] On overlap destory
  (if (not (`self.ActorHasTag` OtherActor "Ignore"))
    (bind _teamid (message `/Game/c013265l/Blueprints/Interfaces/BPI_Teams.I_GetTeam` OtherActor))
    (if (not (`|EnumEquality` _teamid (`self.TeamID`)))
      (`/Engine/EditorBlueprintResources/StandardMacros.DoOnce` false
        (:`Completed`
          (message `/Game/c013265l/Blueprints/Interfaces/BPI_RoundManagement.I_PickupCollected` (`GameplayStatics.GetGameMode`) (`self.TeamID`)))))
    (`self.K2_DestroyActor`)))

(event `/Game/c013265l/Blueprints/Interfaces/BPI_Pickups.I_SpawnPickup`
  (params (TeamID :type "/Game/c013265l/Gameplay/Enum_Teams Enum" :default "NewEnumerator0"))
  ;[1 0.7152 0] Spawn pickup
  (set `self.TeamID` TeamID))

(event `self.ReceiveBeginPlay`
  ;[1 0.6976 0] set sphere collision
  (`KismetSystemLibrary.Delay` 0.5)
  (`PrimitiveComponent.SetCollisionEnabled` (`self.Sphere1`) "QueryOnly"))

(fn `UserConstructionScript`)
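; Pickup actor that grants a timed buff to whatever overlaps it, then destroys itself.
; The construction script derives the buff enum from the display name of the assigned BuffType class, covering damage, speed and mana buffs.
; On sphere overlap, actors implementing BPI_Pickups receive an IBuffAddedMessage with a fixed duration, the enum and the class reference.
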(event `self.Sphere1.OnComponentBeginOverlap`
  (params (OverlappedComponent :type "PrimitiveComponent Object Reference") (OtherActor :type "Actor Object Reference") (OtherComp :type "PrimitiveComponent Object Reference") (OtherBodyIndex :type Integer) (bFromSweep :type Boolean) (SweepResult :type "HitResult Structure (by ref)"))
  (if (`KismetSystemLibrary.DoesImplementInterface` OtherActor "/Game/c013265l/Blueprints/Interfaces/BPI_Pickups.BPI_Pickups_C")
    (message `/Game/c013265l/Blueprints/Interfaces/BPI_Pickups.I_BuffAdded` OtherActor 20.0 null (`self.BuffTypeEnum`) (`self.BuffType`))
    (`self.K2_DestroyActor`)))

(fn `UserConstructionScript`
  (switch `string` (`KismetSystemLibrary.GetClassDisplayName` (`self.BuffType`))
    (:`DamageBuff`
      (set `self.BuffTypeEnum` "NewEnumerator0"))
    (:`SpeedBuff`
      (set `self.BuffTypeEnum` "NewEnumerator1"))
    (:`ManaBuff`
      (set `self.BuffTypeEnum` "NewEnumerator2"))))
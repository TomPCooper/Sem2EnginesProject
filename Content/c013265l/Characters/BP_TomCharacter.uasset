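; BP_TomCharacter is a melee hero Blueprint with a basic attack, three abilities and life steal on damage dealt.
; Ability 1 spawns a team-owned BP_Ability1Tom actor; Ability 2 knocks back and damages nearby other-team pawns.
; Ability 3 starts a timed ultimate boosting speed and life steal, blocking Abilities 1–2, with limited, wider box-overlap attacks.
; Basic attacks lack team checks; the timer setup for line-trace melee is unconnected.
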(event `self.FireAbility1`
  (bind _returnvalue (`self.GetTransform`))
  (if (not (`self.InUltimate`))
    (bind _returnvalue_2 (`|SpawnActorFromClass` "/Game/c013265l/Characters/Abilities/BP_Ability1Tom.BP_Ability1Tom_C" (`KismetMathLibrary.MakeTransform` (`KismetMathLibrary.MakeVector` (.x (.location _returnvalue)) (.y (.location _returnvalue))) (.rotation _returnvalue) (.scale _returnvalue)) "Undefined" "OverrideRootScale" null self))
    (bind _teamid (`/Game/c013265l/Blueprints/Interfaces/BPI_Teams.I_GetTeam`))
    (message `/Game/c013265l/Blueprints/Interfaces/BPI_Abilites.I_SetOwningTeam` _returnvalue_2 _teamid (`self.GetController`))
    (message `/Game/c013265l/Blueprints/Interfaces/BPI_Abilites.I_StartAbility` _returnvalue_2)))

(event `LifeSteal`
  (params (DamageDone :type "Float (double-precision)"))
  (`self.ModifyHealth` (* DamageDone (`self.LifeStealModifier`)) true))

(event `self.FireAbility2`
  (bind _returnvalue (`self.K2_GetActorLocation`))
  (if (not (`self.InUltimate`))
    (bind (_outhits _returnvalue_2) (`KismetSystemLibrary.SphereTraceMultiForObjects` :`Start` _returnvalue :`End` _returnvalue :`Radius` 250.0 :`ObjectTypes` (`|MakeArray` "ObjectTypeQuery3" :!type "EObjectTypeQuery Enum") :`DrawDebugType` "ForDuration"))
    (if _returnvalue_2
      (for _array_element _outhits
        (bind (_bblockinghit _binitialoverlap _time _distance _location _impactpoint _normal _impactnormal _physmat _hitactor) (`GameplayStatics.BreakHitResult` _array_element))
        (`/Engine/EditorBlueprintResources/StandardMacros.IsValid` _hitactor
          (:`Is Valid`
            (bind _teamid (message `/Game/c013265l/Blueprints/Interfaces/BPI_Teams.I_GetTeam` _hitactor))
            (bind _teamid_2 (`/Game/c013265l/Blueprints/Interfaces/BPI_Teams.I_GetTeam`))
            (if (not (`|EnumEquality` _teamid_2 _teamid))
              (`CharacterMovementComponent.AddImpulse` (`self.GetComponentByClass` _hitactor "/Script/Engine.CharacterMovementComponent") (`KismetMathLibrary.ClampVectorSize` (* (- (`self.K2_GetActorLocation` _hitactor) (`self.K2_GetActorLocation`)) (`KismetMathLibrary.RandomFloatInRange` 10.0 16.0)) 0.0 1000.0) true)
              (bind _returnvalue_3 (`GameplayStatics.ApplyDamage` _hitactor 40.0 (`self.GetController`) self "/Game/c013265l/Blueprints/DamageTypes/BP_StandardDamage.BP_StandardDamage_C"))
              (`self.LifeSteal` _returnvalue_3))))))))

(event `self.FireAbility3`
  (set `self.InUltimate` true)
  (`KismetSystemLibrary.K2_SetTimerDelegate` (delegate `EndUltimate`) 6.0)
  (set `CharacterMovementComponent.MaxWalkSpeed` 650.0 (`self.CharacterMovement`))
  (set `self.LifeStealModifier` 0.5))

(event `EndUltimate`
  (set `self.InUltimate` false)
  (set `CharacterMovementComponent.MaxWalkSpeed` 500.0 (`self.CharacterMovement`))
  (set `self.LifeStealModifier` 0.2))

(event `self.FireBasicAttack`
  (set `self.MeleeCounter` 0)
  (if (`self.InUltimate`)
    (if (>= (`self.UltimateCounter`) 3)
      (`self.EndUltimate`)
      (set `self.UltimateCounter` 0)
      (else
        (`/Engine/EditorBlueprintResources/StandardMacros.IncrementInt` (`self.UltimateCounter`)
          (:`  `
            (bind (_outactors _returnvalue) (`KismetSystemLibrary.BoxOverlapActors` (`SceneComponent.K2_GetComponentLocation` (`self.UltimateAttackLoc`)) (200.0 200.0 200.0) (`|MakeArray` "ObjectTypeQuery3" :!type "EObjectTypeQuery Enum")))
            (if _returnvalue
              (for _array_element _outactors
                (bind _returnvalue_2 (`GameplayStatics.ApplyDamage` _array_element 30.0 (`self.GetController`) self "/Game/c013265l/Blueprints/DamageTypes/BP_StandardDamage.BP_StandardDamage_C"))
                (`self.LifeSteal` _returnvalue_2)))))))
    (else
      (`|PlayMontage` (`self.Mesh`) "/Game/c013265l/Characters/Animations/AnimMontage_Melee.AnimMontage_Melee"
        (:`then`
          (bind (_outactors_2 _returnvalue_3) (`KismetSystemLibrary.BoxOverlapActors` (`SceneComponent.K2_GetComponentLocation` (`self.UltimateAttackLoc`)) (100.0 100.0 100.0) (`|MakeArray` "ObjectTypeQuery3" :!type "EObjectTypeQuery Enum")))
          (if _returnvalue_3
            (for _array_element_2 _outactors_2
              (bind _returnvalue_4 (`GameplayStatics.ApplyDamage` _array_element_2 30.0 (`self.GetController`) self "/Game/c013265l/Blueprints/DamageTypes/BP_StandardDamage.BP_StandardDamage_C"))
              (`self.LifeSteal` _returnvalue_4))))))))

(event `StartCollision`
  (bind (_outhit _returnvalue) (`KismetSystemLibrary.LineTraceSingleForObjects` :`End` (+ (0.0 0.0 0.0) (`KismetMathLibrary.MakeVector` 0.0 0.0 (* (.z (`.BoxExtent` (`KismetSystemLibrary.GetComponentBounds` null))) 2.0))) :`ObjectTypes` (`|MakeArray` "ObjectTypeQuery3" :!type "EObjectTypeQuery Enum") :`DrawDebugType` "Persistent"))
  (if _returnvalue
    (bind (_bblockinghit _binitialoverlap _time _distance _location _impactpoint _normal _impactnormal _physmat _hitactor) (`GameplayStatics.BreakHitResult` _outhit))
    (if (`KismetSystemLibrary.DoesImplementInterface` _hitactor "/Game/c013265l/Blueprints/Interfaces/BPI_Damage.BPI_Damage_C")
      (bind _returnvalue_2 (`GameplayStatics.ApplyDamage` _hitactor 20.0 (`self.GetController`) self "/Game/c013265l/Blueprints/DamageTypes/BP_StandardDamage.BP_StandardDamage_C"))
      (`self.LifeSteal` _returnvalue_2)
      (`KismetSystemLibrary.K2_ClearAndInvalidateTimerHandle` (`self.MeleeHandle`) :!label _label)
      (set `self.MeleeCounter` 0))
    (else
      (bind _result (`/Engine/EditorBlueprintResources/StandardMacros.IncrementInt` (`self.MeleeCounter`))
        (:`  `
          (if (>= _result 20)
            (goto _label)))))))

(fn `UserConstructionScript`
  (`parent.UserConstructionScript`))
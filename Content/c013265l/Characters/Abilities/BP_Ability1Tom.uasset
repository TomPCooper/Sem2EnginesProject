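; BP_Ability1Tom is a short-lived area healing ability actor that destroys itself a few seconds after starting.
; While active, a looping timer sphere-overlaps nearby BP_ThirdPersonCharacter pawns around the actor and heals them through ApplyDamage with the BP_HealingDamage type.
; An interface event supplies team and instigating controller, but HealAllies does no team filtering itself.
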(event `/Game/c013265l/Blueprints/Interfaces/BPI_Abilites.I_SetOwningTeam`
  (params (TeamID :type "/Game/c013265l/Gameplay/Enum_Teams Enum" :default "NewEnumerator0") (OwningController :type "Controller Object Reference"))
  (set `self.OwningTeam` TeamID)
  (set `self.Owning Controller` OwningController))

(event `/Game/c013265l/Blueprints/Interfaces/BPI_Abilites.I_StartAbility`
  (`KismetSystemLibrary.K2_SetTimerDelegate` (delegate `HealAllies`) 0.5 true)
  (`KismetSystemLibrary.K2_SetTimerDelegate` (delegate `EndAbility`) 5.0))

(event `EndAbility`
  (`self.K2_DestroyActor`))

(event `HealAllies`
  (bind (_outactors _returnvalue) (`KismetSystemLibrary.SphereOverlapActors` (`self.K2_GetActorLocation`) 300.0 (`|MakeArray` "ObjectTypeQuery3" :!type "EObjectTypeQuery Enum") "/Game/ThirdPerson/Blueprints/BP_ThirdPersonCharacter.BP_ThirdPersonCharacter_C"))
  (if _returnvalue
    (for _array_element _outactors
      (`GameplayStatics.ApplyDamage` _array_element 10.0 (`self.Owning Controller`) self "/Game/c013265l/Blueprints/DamageTypes/BP_HealingDamage.BP_HealingDamage_C"))))

(fn `UserConstructionScript`)
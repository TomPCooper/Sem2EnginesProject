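; BP_TeamPlayerStart is a player start tagged with a team ID.
; Its construction script writes the team's name on a Team text render component and selects that text's color by team.
; It exposes the ID through a team interface getter, while the matching setter is an empty stub that leaves the team unchanged.
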(fn `I_GetTeam`
  (returns (TeamID :type "/Game/c013265l/Gameplay/Enum_Teams Enum"))
  (return (`self.TeamID`)))

(fn `I_SetTeam`
  (params (TeamID :type "/Game/c013265l/Gameplay/Enum_Teams Enum" :default "NewEnumerator0"))
  (return))

(fn `UserConstructionScript`
  (`TextRenderComponent.K2_SetText` (`self.Team`) (`KismetTextLibrary.Conv_StringToText` (`|GetEnumeratorNameAsString` (`self.TeamID`))))
  (`TextRenderComponent.SetTextRenderColor` (`self.Team`) (select `/Game/c013265l/Gameplay/Enum_Teams` (`self.TeamID`) :`NewEnumerator0` (make `Color` :`G` 255) :`NewEnumerator1` (make `Color` :`B` 255) :`NewEnumerator2` (make `Color` :`R` 255))))
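; Domination control point that, while activated via interface, lets Team A or B capture it by standing in its configurable collision box.
; Overlap events identify each player's team through the instigator controller and track team presence and head counts.
; A sole team runs its capture timeline, updating DominationUI progress and time; contested or empty points pause both, retaining progress.
; A finished timeline tells the GameMode to advance the round for that team.
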(event `/Game/c013265l/Blueprints/Interfaces/BPI_Domination.I_SetActiveControlPoint`
  (params (ShouldBeActive :type Boolean))
  (bind _output_get (set `self.IsActive` ShouldBeActive))
  (if _output_get
    _))

(event `self.Collision.OnComponentBeginOverlap`
  (params (OverlappedComponent :type "PrimitiveComponent Object Reference") (OtherActor :type "Actor Object Reference") (OtherComp :type "PrimitiveComponent Object Reference") (OtherBodyIndex :type Integer) (bFromSweep :type Boolean) (SweepResult :type "HitResult Structure (by ref)"))
  (bind _dominationui (`self.DominationUI`))
  (if (`self.IsActive`)
    (if (`KismetSystemLibrary.DoesImplementInterface` OtherActor "/Game/c013265l/Blueprints/Interfaces/BPI_Damage.BPI_Damage_C")
      (bind _teamid (message `/Game/c013265l/Blueprints/Interfaces/BPI_Teams.I_GetTeam` (`self.GetInstigatorController` OtherActor)))
      (bind _output_get (set `self.Team ID` _teamid))
      (switch `/Game/c013265l/Gameplay/Enum_Teams` _output_get
        (:`NewEnumerator1`
          (`/Engine/EditorBlueprintResources/StandardMacros.IncrementInt` (`self.TeamAPlayers`)
            (:`  `
              (set `self.TeamAOnPoint` true))))
        (:`NewEnumerator2`
          (`/Engine/EditorBlueprintResources/StandardMacros.IncrementInt` (`self.TeamBPlayers`)
            (:`  `
              (set `self.TeamBOnPoint` true)))))
      (if (and (`self.TeamAOnPoint`) (`self.TeamBOnPoint`)) :!label _label
        (`self.StopAllProgress`)
        (set `self.Team ID` "NewEnumerator0")
        (else
          (switch `/Game/c013265l/Gameplay/Enum_Teams` (`self.Team ID`)
            (:`NewEnumerator1`
              (`|ExecutionSequence`
                (:`then_0`
                  (bind (_direction _teambprogress _teambtimeleft) (`Timeline|CaptureProgressTeamB` :!via `Stop` :!label _label_2)
                    (:`Update`
                      (`ProgressBar.SetPercent` (`/Game/c013265l/UI/UI_Domination.TeamBProgress` _dominationui) _teambprogress)
                      (`TextBlock.SetText` (`/Game/c013265l/UI/UI_Domination.TextBTime` _dominationui) (`KismetTextLibrary.Conv_DoubleToText` _teambtimeleft "HalfToEven")))
                    (:`Finished`
                      (message `/Game/c013265l/Blueprints/Interfaces/BPI_Domination.I_AdvanceRound` (`GameplayStatics.GetGameMode`) "NewEnumerator2"))))
                (:`then_1`
                  (set `self.Team ID` "NewEnumerator0")
                  (bind (_direction_2 _teamaprogress _teamatimeleft) (`Timeline|CaptureProgressTeamA` :!label _label_3)
                    (:`Update`
                      (`ProgressBar.SetPercent` (`/Game/c013265l/UI/UI_Domination.TeamAProgress` _dominationui) _teamaprogress)
                      (`TextBlock.SetText` (`/Game/c013265l/UI/UI_Domination.TextATime` _dominationui) (`KismetTextLibrary.Conv_DoubleToText` _teamatimeleft "HalfToEven")))
                    (:`Finished`
                      (message `/Game/c013265l/Blueprints/Interfaces/BPI_Domination.I_AdvanceRound` (`GameplayStatics.GetGameMode`) "NewEnumerator1"))))))
            (:`NewEnumerator2`
              (`|ExecutionSequence`
                (:`then_0`
                  (goto _label_3 :!via `Stop`))
                (:`then_1`
                  (set `self.Team ID` "NewEnumerator0")
                  (goto _label_2))))))))))

(event `StartProgressA`
  (goto _label_3))

(event `StopAllProgress`
  (`|ExecutionSequence`
    (:`then_0`
      (goto _label_3 :!via `Stop`))
    (:`then_1`
      (goto _label_2 :!via `Stop`))))

(event `CheckIfShouldProgress`
  (goto _label))

(event `StartProgressB`
  (goto _label_2))

(event `self.Collision.OnComponentEndOverlap`
  (params (OverlappedComponent :type "PrimitiveComponent Object Reference") (OtherActor :type "Actor Object Reference") (OtherComp :type "PrimitiveComponent Object Reference") (OtherBodyIndex :type Integer))
  ;[1 1 1] Check if players have left
  (if (`self.IsActive`)
    (bind _teamid (message `/Game/c013265l/Blueprints/Interfaces/BPI_Teams.I_GetTeam` (`self.GetInstigatorController` OtherActor)))
    (switch `/Game/c013265l/Gameplay/Enum_Teams` _teamid
      (:`NewEnumerator1`
        (`/Engine/EditorBlueprintResources/StandardMacros.DecrementInt` (`self.TeamAPlayers`)
          (:`  `
            _)))
      (:`NewEnumerator2`
        (`/Engine/EditorBlueprintResources/StandardMacros.DecrementInt` (`self.TeamBPlayers`)
          (:`  `
            _))))
    (if (`KismetArrayLibrary.Array_IsEmpty` (`PrimitiveComponent.GetOverlappingActors` (`self.Collision`) "/Game/ThirdPerson/Blueprints/BP_ThirdPersonCharacter.BP_ThirdPersonCharacter_C"))
      (`self.StopAllProgress`)
      (else
        (`|ExecutionSequence`
          (:`then_0`
            (if (> (`self.TeamAPlayers`) 0)
              (set `self.Team ID` "NewEnumerator1")
              (else
                (set `self.TeamAOnPoint` false))))
          (:`then_1`
            (if (> (`self.TeamBPlayers`) 0)
              (set `self.Team ID` "NewEnumerator2")
              (else
                (set `self.TeamBOnPoint` false))))
          (:`then_2`
            (`self.CheckIfShouldProgress`)))))))

(fn `UserConstructionScript`
  (`BoxComponent.SetBoxExtent` (`self.Collision`) (`self.BoxExtent`) true))
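; Domination capture point whose box collision, sized in the construction script, tracks Team A and Team B players standing on it.
; On overlap, damageable actors report their team via BPI_Damage; the first starts that team's capture timeline, while any arrival on an occupied point stops both.
; On exit, counts decrement and occupancy flags clear at zero only if characters still overlap, without restarting progress.
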(event `StartProgressA`
  (`Timeline|CaptureProgressTeamA` :!label _label))

(event `self.Collision.OnComponentBeginOverlap`
  (params (OverlappedComponent :type "PrimitiveComponent Object Reference") (OtherActor :type "Actor Object Reference") (OtherComp :type "PrimitiveComponent Object Reference") (OtherBodyIndex :type Integer) (bFromSweep :type Boolean) (SweepResult :type "HitResult Structure (by ref)"))
  (if (`KismetSystemLibrary.DoesImplementInterface` OtherActor "/Game/c013265l/Blueprints/Interfaces/BPI_Damage.BPI_Damage_C")
    (bind _teamid (message `/Game/c013265l/Blueprints/Interfaces/BPI_Teams.I_GetTeam` OtherActor))
    (if (or (`self.TeamAOnPoint`) (`self.TeamBOnPoint`))
      (`self.StopAllProgress`)
      (else
        (bind _output_get (set `self.Team ID` _teamid))
        (switch `/Game/c013265l/Gameplay/Enum_Teams` _output_get
          (:`NewEnumerator1`
            (`/Engine/EditorBlueprintResources/StandardMacros.IncrementInt` (`self.TeamAPlayers`)
              (:`  `
                (set `self.TeamAOnPoint` true)
                (goto _label))))
          (:`NewEnumerator2`
            (`/Engine/EditorBlueprintResources/StandardMacros.IncrementInt` (`self.TeamBPlayers`)
              (:`  `
                (set `self.TeamBOnPoint` true)
                (`Timeline|CaptureProgressTeamB` :!label _label_2)))))))))

(event `StopAllProgress`
  (`|ExecutionSequence`
    (:`then_0`
      (goto _label :!via `Stop`))
    (:`then_1`
      (goto _label_2 :!via `Stop`))))

(event `StartProgressB`
  (goto _label_2))

(event `self.Collision.OnComponentEndOverlap`
  (params (OverlappedComponent :type "PrimitiveComponent Object Reference") (OtherActor :type "Actor Object Reference") (OtherComp :type "PrimitiveComponent Object Reference") (OtherBodyIndex :type Integer))
  (bind _teamid (message `/Game/c013265l/Blueprints/Interfaces/BPI_Teams.I_GetTeam` OtherActor))
  (switch `/Game/c013265l/Gameplay/Enum_Teams` _teamid
    (:`NewEnumerator1`
      (bind _result (`/Engine/EditorBlueprintResources/StandardMacros.DecrementInt` (`self.TeamAPlayers`))
        (:`  `
          _)))
    (:`NewEnumerator2`
      (bind _result_2 (`/Engine/EditorBlueprintResources/StandardMacros.DecrementInt` (`self.TeamBPlayers`))
        (:`  `
          _))))
  (if (not (`KismetArrayLibrary.Array_IsEmpty` (`PrimitiveComponent.GetOverlappingActors` (`self.Collision`) "/Game/ThirdPerson/Blueprints/BP_ThirdPersonCharacter.BP_ThirdPersonCharacter_C")))
    (`|ExecutionSequence`
      (:`then_0`
        (if (not (> _result 0))
          (set `self.TeamAOnPoint` false)))
      (:`then_1`
        (if (not (> _result_2 0))
          (set `self.TeamBOnPoint` false))))))

(fn `UserConstructionScript`
  (`BoxComponent.SetBoxExtent` (`self.Collision`) (`self.BoxExtent`) true))
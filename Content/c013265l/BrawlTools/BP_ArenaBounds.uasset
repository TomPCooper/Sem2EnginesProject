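; BP_ArenaBounds is a spherical arena boundary that shrinks on command and damages team actors outside it.
; The IStartArenaShrinking event plays a timeline that scales the sphere radius down to a minimum size, with the initial radius set in the Construction Script.
; Overlap events track exited actors implementing BPI_Teams, driving a looping timer that applies periodic damage until all have re-entered.
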(event `/Game/c013265l/Blueprints/Interfaces/BPI_Brawl.I_StartArenaShrinking`
  (bind _sphereradius (`self.SphereRadius`))
  (bind (_direction _alpha) (`Timeline|RadiusShrinking`)
    (:`Update`
      (`SphereComponent.SetSphereRadius` (`self.Sphere`) (`KismetMathLibrary.FClamp` (* _alpha _sphereradius) (`self.MinimumArenaSize`) _sphereradius) true))))

(event `self.Sphere.OnComponentEndOverlap`
  (params (OverlappedComponent :type "PrimitiveComponent Object Reference") (OtherActor :type "Actor Object Reference") (OtherComp :type "PrimitiveComponent Object Reference") (OtherBodyIndex :type Integer))
  (if (`KismetSystemLibrary.DoesImplementInterface` OtherActor "/Game/c013265l/Blueprints/Interfaces/BPI_Teams.BPI_Teams_C")
    (`KismetArrayLibrary.Array_AddUnique` (`self.ActorstoDamage`) OtherActor)
    (bind _returnvalue (`KismetSystemLibrary.K2_SetTimerDelegate` (`|CreateDelegate` :!event `DamagePlayer`) 1.0 true))
    (set `self.DamageHandle` _returnvalue)))

(event `DamagePlayer`
  (for _array_element (`self.ActorstoDamage`)
    (`GameplayStatics.ApplyDamage` _array_element 20.0 null null "/Game/c013265l/Blueprints/DamageTypes/BP_StandardDamage.BP_StandardDamage_C")))

(event `self.Sphere.OnComponentBeginOverlap`
  (params (OverlappedComponent :type "PrimitiveComponent Object Reference") (OtherActor :type "Actor Object Reference") (OtherComp :type "PrimitiveComponent Object Reference") (OtherBodyIndex :type Integer) (bFromSweep :type Boolean) (SweepResult :type "HitResult Structure (by ref)"))
  (bind _actorstodamage (`self.ActorstoDamage`))
  (if (`KismetSystemLibrary.DoesImplementInterface` OtherActor "/Game/c013265l/Blueprints/Interfaces/BPI_Teams.BPI_Teams_C")
    (`KismetArrayLibrary.Array_RemoveItem` _actorstodamage OtherActor)
    (if (<= (`KismetArrayLibrary.Array_Length` _actorstodamage) 0)
      (`KismetSystemLibrary.K2_ClearAndInvalidateTimerHandle` (`self.DamageHandle`)))))

(fn `UserConstructionScript`
  (`SphereComponent.SetSphereRadius` (`self.Sphere`) (`self.SphereRadius`) true))
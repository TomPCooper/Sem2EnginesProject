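; BP_Flag is a team-owned capture-the-flag actor that an opposing player picks up by touch.
; A team interface event stores the owning team and applies its material to the Cylinder.
; Capsule overlap by a differing team calls FlagPickup, which records the holder, hides the mesh and disables collision.
; FlagReset, uncalled here, restores collision and pickup state but leaves the mesh hidden.
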(event `/Game/c013265l/Blueprints/Interfaces/BPI_Teams.I_SetTeam`
  (params (TeamID :type "/Game/c013265l/Gameplay/Enum_Teams Enum" :default "NewEnumerator0"))
  ;[1 1 1] Flag Initiate
  (bind _output_get (set `self.FlagTeam` TeamID))
  (`KismetSystemLibrary.PrintString` "flag a")
  (switch `/Game/c013265l/Gameplay/Enum_Teams` _output_get
    (:`NewEnumerator1`
      (`KismetSystemLibrary.PrintString` "flag a")
      (`PrimitiveComponent.SetMaterial` (`self.Cylinder`) 0 "/Game/b017383l/CTF/M_FlagA.M_FlagA"))
    (:`NewEnumerator2`
      (`KismetSystemLibrary.PrintString` "flag b")
      (`PrimitiveComponent.SetMaterial` (`self.Cylinder`) 0 "/Game/b017383l/CTF/M_FlagB.M_FlagB"))))

(event `self.Capsule.OnComponentBeginOverlap`
  (params (OverlappedComponent :type "PrimitiveComponent Object Reference") (OtherActor :type "Actor Object Reference") (OtherComp :type "PrimitiveComponent Object Reference") (OtherBodyIndex :type Integer) (bFromSweep :type Boolean) (SweepResult :type "HitResult Structure (by ref)"))
  ;[1 1 1] Picking up flag
  (bind _teamid (message `/Game/c013265l/Blueprints/Interfaces/BPI_Teams.I_GetTeam` OtherActor))
  (if (`|EnumInequality` _teamid (`self.FlagTeam`))
    (if (not (`self.IsPickedUp`))
      (`self.FlagPickup` (cast `Pawn` OtherActor :!pure true)))))

(fn `Flag Reset`
  (bind _cylinder (`self.Cylinder`))
  (set `self.FlagHolder` (`self.HolderReset`))
  (`SceneComponent.SetVisibility` _cylinder false false)
  (`PrimitiveComponent.SetCollisionEnabled` _cylinder "QueryAndPhysics")
  (`PrimitiveComponent.SetCollisionEnabled` (`self.Capsule`) "QueryAndPhysics")
  (`KismetSystemLibrary.PrintString` "flag reset")
  (set `self.IsPickedUp` false))

(fn `FlagPickup`
  (params (Player :type "Pawn Object Reference"))
  (bind _cylinder (`self.Cylinder`))
  (set `self.FlagHolder` Player)
  (`SceneComponent.SetVisibility` _cylinder false false)
  (`PrimitiveComponent.SetCollisionEnabled` _cylinder "NoCollision")
  (`PrimitiveComponent.SetCollisionEnabled` (`self.Capsule`) "NoCollision")
  (`KismetSystemLibrary.PrintString` "Flag acquired")
  (set `self.IsPickedUp` true))

(fn `I_GetPlayerData`
  (returns (PlayerData :type "/Game/c013265l/Structs/S_PlayerData Structure"))
  (return))

(fn `I_GetTeam`
  (returns (TeamID :type "/Game/c013265l/Gameplay/Enum_Teams Enum"))
  (return "NewEnumerator0"))

(fn `UserConstructionScript`)
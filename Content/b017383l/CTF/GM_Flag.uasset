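; Game mode for local capture-the-flag with up to four players in two teams on a shared map camera.
; It creates players from GameInstance data, spawns pawns and flags at team spawns, and steps GS_GameStateBase from pre-game through timed play to the menu.
; Interface events handle respawns, flag resets and deposit scoring through one shared CarryingFlag boolean.
; Reaching three points only sets ScoreAchieved; the end check runs on time-up.
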(event `self.ReceiveBeginPlay`
  ;[1 1 1] Start Game
  (set `self.GameInstance` (cast `/Game/c013265l/Blueprints/GameInstances/GameInstance` (`GameplayStatics.GetGameInstance`) :!pure true))
  (bind _returnvalue (`GameplayStatics.GetActorOfClass` "/Game/c013265l/Blueprints/BP_Camera.BP_Camera_C"))
  (set `self.MapCamera` _returnvalue)
  (`self.Init`))

(event `Init`
  ;[1 1 1] Initiate
  (`self.SetUpController`)
  (`self.SpawnCharacters`)
  (`self.BindToGameState`)
  (`/Game/c013265l/Blueprints/PlayerControllers/PC_Game.Init` (`self.GamePlayControllers`))
  (`self.SetScore0`)
  (`self.InitFlags`)
  (`KismetSystemLibrary.Delay` 2.0)
  (`/Game/c013265l/Blueprints/GameStates/GS_GameStateBase.UpdateState` (`self.GS_GameState`) "NewEnumerator1" "NewEnumerator0"))

(event `BindToGameState`
  ;[1 1 1] Game State
  (bind _output_get (set `self.GS_GameState` (cast `/Game/c013265l/Blueprints/GameStates/GS_GameStateBase` (`GameplayStatics.GetGameState`) :!pure true)))
  (add `/Game/c013265l/Blueprints/GameStates/GS_GameStateBase.GameStateChanged` _output_get (`|CreateDelegate` :!event `GameStateChanged`)))

(event `InitFlags`
  ;[1 1 1] Flag Initiation
  (`self.Spawn Flags`))

(event `/Game/c013265l/Blueprints/Interfaces/BPI_RoundManagement.I_PlayerDeath`
  (params (TeamID :type "/Game/c013265l/Gameplay/Enum_Teams Enum" :default "NewEnumerator0") (DeadPawn :type "Pawn Object Reference"))
  ;[1 1 1] Player Mechanics
  (`self.Death Mechanics` DeadPawn)
  (bind _aspc_game (cast `/Game/c013265l/Blueprints/PlayerControllers/PC_Game` (`Pawn.GetController` DeadPawn)))
  (`self.I_RespawnPlayer` _aspc_game TeamID))

(event `GameStateChanged`
  (params (CurrentGameState :type "/Game/c013265l/Blueprints/Enumerators/E_GameState Enum" :default "NewEnumerator0"))
  ;[1 1 1] Game State
  (switch `/Game/c013265l/Blueprints/Enumerators/E_GameState` CurrentGameState
    (:`NewEnumerator1`
      (`KismetSystemLibrary.PrintString` "Pre Game")
      (`KismetSystemLibrary.Delay` 3.0)
      (`/Game/c013265l/Blueprints/GameStates/GS_GameStateBase.UpdateState` (`self.GS_GameState`) "NewEnumerator2" "NewEnumerator4"))
    (:`NewEnumerator2`
      (`KismetSystemLibrary.PrintString` "InGame")
      (`KismetSystemLibrary.K2_SetTimerDelegate` (`|CreateDelegate` :!event `TimeUp`) 60.0))
    (:`NewEnumerator3`
      (`KismetSystemLibrary.PrintString` "EndingGame")
      (`self.EndGame`))))

(event `self.I_RespawnPlayer`
  (params (Controller :type "/Game/c013265l/Blueprints/PlayerControllers/PC_Game Object Reference") (TeamID :type "/Game/c013265l/Gameplay/Enum_Teams Enum" :default "NewEnumerator0"))
  ;[1 1 1] Player Mechanics
  (`self.RespawnPlayer` Controller TeamID))

(event `self.I_FlagOverlap`
  (params (PawnOverlap :type "Pawn Object Reference") (`Spawn Overlap` :type "/Game/b017383l/CTF/BP_FlagSpawn Object Reference"))
  ;[1 1 1] Player Mechanics
  (`self.Deposit Mechanics` PawnOverlap `Spawn Overlap`))

(event `TimeUp`
  ;[1 1 1] EndGame
  (set `self.HasTimeRanOut` true)
  (`self.CanEndGame`))

(event `self.I_FlagPickup`
  (params (isCarried :type Boolean))
  ;[1 1 1] Player Mechanics
  (set `self.CarryingFlag` true)
  (`KismetSystemLibrary.PrintString` "carrying flag true"))

(event `self.I_FlagDrop`
  (params (isCarried :type Boolean))
  ;[1 1 1] Player Mechanics
  (set `self.CarryingFlag` false)
  (`KismetSystemLibrary.PrintString` "carrying flag false"))

(event `EndGame`
  ;[1 1 1] EndGame
  (`KismetSystemLibrary.Delay` 3.0)
  (`/Game/c013265l/Blueprints/FucntionLibraries/BPL_GamePlay.RemoveAllPlayers`)
  (`GameplayStatics.OpenLevel` "Menu_Main"))

(event `self.K2_PostLogin`
  (params (NewPlayer :type "PlayerController Object Reference"))
  ;[1 1 1] Login/Logout Events
  (bind _aspc_game (cast `/Game/c013265l/Blueprints/PlayerControllers/PC_Game` NewPlayer))
  (`KismetArrayLibrary.Array_Add` (`self.GamePlayControllers`) _aspc_game))

(event `self.K2_OnLogout`
  (params (ExitingController :type "Controller Object Reference"))
  ;[1 1 1] Login/Logout Events
  (bind _aspc_game (cast `/Game/c013265l/Blueprints/PlayerControllers/PC_Game` ExitingController))
  (`KismetArrayLibrary.Array_RemoveItem` (`self.GamePlayControllers`) _aspc_game)
  (`KismetArrayLibrary.Array_RemoveItem` (`self.TeamA_Players`) _aspc_game)
  (`KismetArrayLibrary.Array_RemoveItem` (`self.TeamB_Players`) _aspc_game))

(fn `AddToTeamLists`
  (params (GameplayController :type "/Game/c013265l/Blueprints/PlayerControllers/PC_Game Object Reference"))
  (bind _teamid (message `/Game/c013265l/Blueprints/Interfaces/BPI_Teams.I_GetTeam` GameplayController))
  (switch `/Game/c013265l/Gameplay/Enum_Teams` _teamid
    (:`NewEnumerator1`
      (`KismetArrayLibrary.Array_Add` (`self.TeamA_Players`) GameplayController))
    (:`NewEnumerator2`
      (`KismetArrayLibrary.Array_Add` (`self.TeamB_Players`) GameplayController))))

(fn `CanEndGame`
  (if (or (`self.HasTimeRanOut`) (`self.Score Achieved`))
    (`/Game/c013265l/Blueprints/GameStates/GS_GameStateBase.UpdateState` (`self.GS_GameState`) "NewEnumerator3" "NewEnumerator4")))

(fn `CheckScore`
  (if (>= (`self.TeamA_Score`) 3)
    (set `self.Score Achieved` true :!label _label)
    (elif (>= (`self.TeamB_Score`) 3)
      (goto _label))))

(fn `ChoosePlayerStart`
  (params (Player :type "Controller Object Reference"))
  (returns (ReturnValue :type "Actor Object Reference"))
  (return null))

(fn `Death Mechanics`
  (params (DeadPlayer :type "Pawn Object Reference"))
  (bind _teamid (message `/Game/c013265l/Blueprints/Interfaces/BPI_Teams.I_GetTeam` DeadPlayer))
  (if (`self.CarryingFlag`)
    (`KismetSystemLibrary.PrintString` "flag found")
    (for _array_element (`self.Flags`)
      (if (`|EnumInequality` _teamid (`/Game/b017383l/CTF/BP_Flag.FlagTeam` _array_element))
        (`/Game/b017383l/CTF/BP_Flag.Flag Reset` _array_element)
        (`self.I_FlagDrop` false)))
    (else
      (`KismetSystemLibrary.PrintString` "no flag found"))))

(fn `Deposit Mechanics`
  (params (OverlapPlayer :type "Pawn Object Reference") (OverlapSpawn :type "/Game/b017383l/CTF/BP_FlagSpawn Object Reference"))
  (locals (CurrentTeam :type "/Game/c013265l/Gameplay/Enum_Teams Enum" :default "NewEnumerator0"))
  (bind _teamid (message `/Game/c013265l/Blueprints/Interfaces/BPI_Teams.I_GetTeam` OverlapPlayer))
  (bind _teamid_2 (message `/Game/c013265l/Blueprints/Interfaces/BPI_Teams.I_GetTeam` OverlapSpawn))
  (if (`|EnumEquality` _teamid _teamid_2)
    (`KismetSystemLibrary.PrintString` "match found")
    (if (`self.CarryingFlag`)
      (`KismetSystemLibrary.PrintString` "flag found")
      (bind _output_get (set `local.CurrentTeam` _teamid))
      (if (`|EnumEquality` _output_get "NewEnumerator1")
        (`KismetSystemLibrary.PrintString` "is team a")
        (bind _result (`/Engine/EditorBlueprintResources/StandardMacros.IncrementInt` (`self.TeamA_Score`))
          (:`  `
            (set `self.TeamA_Score` _result)
            (`self.I_FlagDrop` false)
            (`KismetSystemLibrary.PrintString` "team A score +1")))
        (else
          (`KismetSystemLibrary.PrintString` "is team b")
          (bind _result_2 (`/Engine/EditorBlueprintResources/StandardMacros.IncrementInt` (`self.TeamB_Score`))
            (:`  `
              (set `self.TeamB_Score` _result_2)
              (`self.I_FlagDrop` false)
              (`KismetSystemLibrary.PrintString` "team B score +1")))))
      (`self.CheckScore`)
      (else
        (`KismetSystemLibrary.PrintString` "no flag found")))
    (else
      (`KismetSystemLibrary.PrintString` "no match found"))))

(fn `I_GetCharacterStats`
  (returns (CharacterStats :type "/Game/c013265l/Blueprints/StructsData/S_CharacterStats Structure"))
  (return))

(fn `I_GetPlayerData`
  (returns (PlayerData :type "/Game/c013265l/Structs/S_PlayerData Structure"))
  (return))

(fn `I_GetTeam`
  (returns (TeamID :type "/Game/c013265l/Gameplay/Enum_Teams Enum"))
  (return "NewEnumerator0"))

(fn `RespawnPlayer`
  (params (Controller :type "/Game/c013265l/Blueprints/PlayerControllers/PC_Game Object Reference") (TeamID :type "/Game/c013265l/Gameplay/Enum_Teams Enum" :default "NewEnumerator0"))
  (bind _playerdata (message `/Game/c013265l/Blueprints/Interfaces/BPI_Teams.I_GetPlayerData` Controller))
  (bind ((`PlayerClass_13_AB63BDD64175B900ED43C68475968EA3` _playerclass) (`TeamID_16_C95AF1994DF53F697565858AC86BB26E` _teamid)) (break `/Game/c013265l/Structs/S_PlayerData` _playerdata))
  (bind _returnvalue (`|SpawnActorFromClass` _playerclass (`self.GetTransform` (`self.SelectPlayerStart` _teamid)) "AdjustIfPossibleButAlwaysSpawn" "OverrideRootScale" null null))
  (`Controller.Possess` Controller _returnvalue)
  (message `/Game/c013265l/Blueprints/Interfaces/BPI_PawnCommunication.I_SetPawnTeam` _returnvalue _teamid)
  (`PlayerController.SetViewTargetWithBlend` Controller (`self.MapCamera`) 0.0 "VTBlend_Linear" 0.0 false))

(fn `SelectPlayerStart`
  (params (TeamID :type "/Game/c013265l/Gameplay/Enum_Teams Enum" :default "NewEnumerator0"))
  (returns (StartActor :type "/Game/c013265l/Gameplay/BP_TeamPlayerStart Object Reference"))
  (locals (L_SpawnPointActors :type "Array of /Game/c013265l/Gameplay/BP_TeamPlayerStart Object Reference"))
  (bind _outactors (`GameplayStatics.GetAllActorsOfClass` "/Game/c013265l/Gameplay/BP_TeamPlayerStart.BP_TeamPlayerStart_C"))
  (for _array_element _outactors
    (bind _teamid (message `/Game/c013265l/Blueprints/Interfaces/BPI_Teams.I_GetTeam` _array_element))
    (if (`|EnumEquality` _teamid TeamID)
      (`KismetArrayLibrary.Array_Add` (`local.L_SpawnPointActors`) _array_element)))
  (if (!= (`KismetArrayLibrary.Array_Length` (`local.L_SpawnPointActors`)) 0)
    (return (`KismetArrayLibrary.Array_Random` (`local.L_SpawnPointActors`)))
    (else
      (bind _returnvalue (`GameplayStatics.GetActorOfClass` "/Game/c013265l/Gameplay/BP_TeamPlayerStart.BP_TeamPlayerStart_C"))
      (return _returnvalue))))

(fn `SetScore0`
  (set `self.TeamA_Score` 0)
  (set `self.TeamB_Score` 0))

(fn `SetUpController`
  (bind _gameinstance (`self.GameInstance`))
  (`GameplayStatics.RemovePlayer` (`GameplayStatics.GetPlayerController` 0))
  (for _index (range 4)
    (bind _returnvalue (select `int` _index :`0` (`/Game/c013265l/Blueprints/GameInstances/GameInstance.Player0_data` _gameinstance) :`1` (`/Game/c013265l/Blueprints/GameInstances/GameInstance.Player1_data` _gameinstance) :`2` (`/Game/c013265l/Blueprints/GameInstances/GameInstance.Player2_data` _gameinstance) :`3` (`/Game/c013265l/Blueprints/GameInstances/GameInstance.Player3_data` _gameinstance)))
    (bind ((`PlayerID_2_B9C8EF28415CAA77CC6887A2B3E5FC49` _playerid) (`PlayerClass_13_AB63BDD64175B900ED43C68475968EA3` _playerclass) (`IsActive_19_07E58887427E7C144A22AE87F1E11D74` _isactive)) (break `/Game/c013265l/Structs/S_PlayerData` _returnvalue))
    (if _isactive
      (bind _returnvalue_2 (`GameplayStatics.CreatePlayer` _playerid))
      (message `/Game/c013265l/Blueprints/Interfaces/BPI_Teams.I_SetPlayerData` _returnvalue_2 _returnvalue)
      (`self.AddToTeamLists` (cast `/Game/c013265l/Blueprints/PlayerControllers/PC_Game` _returnvalue_2 :!pure true)))))

(fn `Spawn Flags`
  (returns (Flags :type "Array of /Game/b017383l/CTF/BP_Flag Object Reference"))
  (locals (`Current Spawn` :type "/Game/b017383l/CTF/BP_FlagSpawn Object Reference"))
  (bind _outactors (`GameplayStatics.GetAllActorsOfClass` "/Game/b017383l/CTF/BP_FlagSpawn.BP_FlagSpawn_C"))
  (set `self.Flag Spawns` _outactors)
  (for _array_element _outactors
    (bind _teamid (message `/Game/c013265l/Blueprints/Interfaces/BPI_Teams.I_GetTeam` _array_element))
    (bind _returnvalue (`|SpawnActorFromClass` "/Game/b017383l/CTF/BP_Flag.BP_Flag_C" (`self.GetTransform` _array_element) "AlwaysSpawn" "OverrideRootScale" null null))
    (message `/Game/c013265l/Blueprints/Interfaces/BPI_Teams.I_SetTeam` _returnvalue _teamid)
    (`KismetArrayLibrary.Array_Add` (`self.Flags`) _returnvalue))
  (return (`self.Flags`)))

(fn `SpawnCharacters`
  (for _array_element (`self.GamePlayControllers`)
    (bind _playerdata (message `/Game/c013265l/Blueprints/Interfaces/BPI_Teams.I_GetPlayerData` _array_element))
    (bind ((`PlayerClass_13_AB63BDD64175B900ED43C68475968EA3` _playerclass) (`TeamID_16_C95AF1994DF53F697565858AC86BB26E` _teamid)) (break `/Game/c013265l/Structs/S_PlayerData` _playerdata))
    (bind _returnvalue (`|SpawnActorFromClass` _playerclass (`self.GetTransform` (`self.SelectPlayerStart` _teamid)) "AdjustIfPossibleButAlwaysSpawn" "OverrideRootScale" null null))
    (`Controller.Possess` _array_element _returnvalue)
    (message `/Game/c013265l/Blueprints/Interfaces/BPI_PawnCommunication.I_SetPawnTeam` _returnvalue _teamid)
    (`PlayerController.SetViewTargetWithBlend` _array_element (`self.MapCamera`) 0.0 "VTBlend_Linear" 0.0 false)))

(fn `UserConstructionScript`)
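; Capture-the-flag game mode for local multiplayer that runs team setup and match flow through to a return to the main menu.
; Controller setup reads GameInstance player data, though BeginPlay passes zero players.
; Helpers spawn pawns at random team starts under a shared map camera, and flags with FlipFlop-alternated teams.
; GameState change events drive delayed Pre-Game, timed In-Game and Post-Game phases.
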(event `self.ReceiveBeginPlay`
  ;[1 1 1] Start Game Setup
  (set `self.Game Instance` (cast `/Game/c013265l/Blueprints/GameInstances/GameInstance` (`GameplayStatics.GetGameInstance`) :!pure true))
  (bind _returnvalue (`GameplayStatics.GetActorOfClass` "/Game/c013265l/Blueprints/BP_Camera.BP_Camera_C"))
  (set `self.MapCam` _returnvalue)
  (`self.InitCTF`))

(event `InitCTF`
  ;[1 1 1] Initiate Game Mode
  (`self.SetupController` 0)
  (`self.Spawn Characters`)
  (`self.BindToGameState`)
  (`/Game/c013265l/Blueprints/PlayerControllers/PC_Game.Init` (`self.PlayerControllers`))
  (`self.InitFlags`)
  (`KismetSystemLibrary.Delay` 2.0)
  (`/Game/c013265l/Blueprints/GameStates/GS_GameStateBase.UpdateState` (`self.GS Game State`) "NewEnumerator1"))

(event `BindToGameState`
  ;[1 1 1] Game State Management
  (bind _output_get (set `self.GS Game State` (cast `/Game/c013265l/Blueprints/GameStates/GS_GameStateBase` (`GameplayStatics.GetGameState`) :!pure true)))
  (add `/Game/c013265l/Blueprints/GameStates/GS_GameStateBase.GameStateChanged` _output_get (`|CreateDelegate` :!event `GameStateChanged`)))

(event `InitFlags`
  (bind _flags (`self.Spawn Flags`))
  (for _array_element _flags
    (`/Game/b017383l/CTF/BP_Flag.FlagInit` _array_element)))

(event `GameStateChanged`
  (params (CurrentGameState :type "/Game/c013265l/Blueprints/Enumerators/E_GameState Enum" :default "NewEnumerator0"))
  ;[1 1 1] Game State Management
  (switch `/Game/c013265l/Blueprints/Enumerators/E_GameState` CurrentGameState
    (:`NewEnumerator1`
      (`KismetSystemLibrary.PrintString` "Pre-Game")
      (`KismetSystemLibrary.Delay` 3.0)
      (`/Game/c013265l/Blueprints/GameStates/GS_GameStateBase.UpdateState` (`self.GS Game State`) "NewEnumerator2"))
    (:`NewEnumerator2`
      (`KismetSystemLibrary.PrintString` "In Game")
      (`KismetSystemLibrary.K2_SetTimerDelegate` (`|CreateDelegate` :!event `TimeUp`) 30.0))
    (:`NewEnumerator3`
      (`KismetSystemLibrary.PrintString` "Ending Game")
      (`self.End Game`))))

(event `TimeUp`
  ;[1 1 1] Game State Management
  (set `self.TimeHasRanOut` true)
  (`self.CanEndGame`))

(event `OnPostLogin`)

(event `OnLogout`)

(event `End Game`
  ;[1 1 1] Game State Management
  (`KismetSystemLibrary.Delay` 3.0)
  (`/Game/c013265l/Blueprints/FucntionLibraries/BPL_GamePlay.RemoveAllPlayers`)
  (`GameplayStatics.OpenLevel` "Menu_Main"))

(fn `AddToTeamLists`
  (params (GameplayController :type "/Game/c013265l/Blueprints/PlayerControllers/PC_Game Object Reference"))
  (bind _teamid (message `/Game/c013265l/Blueprints/Interfaces/BPI_Teams.I_GetTeam` GameplayController))
  (switch `/Game/c013265l/Gameplay/Enum_Teams` _teamid
    (:`NewEnumerator1`
      (`KismetArrayLibrary.Array_Add` (`self.TeamA_Players`) GameplayController))
    (:`NewEnumerator2`
      (`KismetArrayLibrary.Array_Add` (`self.TeamB_Players`) GameplayController))))

(fn `CanEndGame`
  (if (or (`self.TimeHasRanOut`) (`self.ThreeWins`))
    (`/Game/c013265l/Blueprints/GameStates/GS_GameStateBase.UpdateState` (`self.GS Game State`) "NewEnumerator3")))

(fn `SelectPlayerSpawn`
  (params (TeamID :type "/Game/c013265l/Gameplay/Enum_Teams Enum" :default "NewEnumerator0"))
  (returns (StartActor :type "/Game/c013265l/Gameplay/BP_TeamPlayerStart Object Reference"))
  (bind _outactors (`GameplayStatics.GetAllActorsOfClass` "/Game/c013265l/Gameplay/BP_TeamPlayerStart.BP_TeamPlayerStart_C"))
  (for _array_element _outactors
    (bind _teamid (message `/Game/c013265l/Blueprints/Interfaces/BPI_Teams.I_GetTeam` _array_element))
    (if (`|EnumEquality` _teamid TeamID)
      (`KismetArrayLibrary.Array_Add` (`self.L_SpawnPointActors`) _array_element)))
  (if (!= (`KismetArrayLibrary.Array_Length` (`self.L_SpawnPointActors`)) 0)
    (return (`KismetArrayLibrary.Array_Random` (`self.L_SpawnPointActors`)))
    (else
      (bind _returnvalue (`GameplayStatics.GetActorOfClass` "/Game/c013265l/Gameplay/BP_TeamPlayerStart.BP_TeamPlayerStart_C"))
      (return _returnvalue))))

(fn `SelectPlayerStart`
  (params (TeamID :type "/Game/c013265l/Gameplay/Enum_Teams Enum" :default "NewEnumerator0"))
  (returns (StartActor :type "/Game/c013265l/Gameplay/BP_TeamPlayerStart Object Reference"))
  (bind _outactors (`GameplayStatics.GetAllActorsOfClass` "/Game/c013265l/Gameplay/BP_TeamPlayerStart.BP_TeamPlayerStart_C"))
  (for _array_element _outactors
    (bind _teamid (message `/Game/c013265l/Blueprints/Interfaces/BPI_Teams.I_GetTeam` _array_element))
    (if (`|EnumEquality` _teamid TeamID)
      (`KismetArrayLibrary.Array_Add` (`self.L_SpawnPointActors`) _array_element)))
  (if (!= (`KismetArrayLibrary.Array_Length` (`self.L_SpawnPointActors`)) 0)
    (return (`KismetArrayLibrary.Array_Random` (`self.L_SpawnPointActors`)))
    (else
      (bind _returnvalue (`GameplayStatics.GetActorOfClass` "/Game/c013265l/Gameplay/BP_TeamPlayerStart.BP_TeamPlayerStart_C"))
      (return _returnvalue))))

(fn `Setup Controller Instance`
  (bind _game_instance (`self.Game Instance`))
  (`GameplayStatics.RemovePlayer` (`GameplayStatics.GetPlayerController` 0))
  (for _index (range 4)
    (bind _returnvalue (select `int` _index :`0` (`/Game/c013265l/Blueprints/GameInstances/GameInstance.Player0_data` _game_instance) :`1` (`/Game/c013265l/Blueprints/GameInstances/GameInstance.Player1_data` _game_instance) :`2` (`/Game/c013265l/Blueprints/GameInstances/GameInstance.Player2_data` _game_instance) :`3` (`/Game/c013265l/Blueprints/GameInstances/GameInstance.Player3_data` _game_instance)))
    (bind ((`PlayerID_2_B9C8EF28415CAA77CC6887A2B3E5FC49` _playerid) (`PlayerClass_13_AB63BDD64175B900ED43C68475968EA3` _playerclass) (`IsActive_19_07E58887427E7C144A22AE87F1E11D74` _isactive)) (break `/Game/c013265l/Structs/S_PlayerData` _returnvalue))
    (if _isactive
      (bind _returnvalue_2 (`GameplayStatics.CreatePlayer` _playerid))
      (message `/Game/c013265l/Blueprints/Interfaces/BPI_Teams.I_SetPlayerData` _returnvalue_2 _returnvalue)
      (`self.AddToTeamLists` (cast `/Game/c013265l/Blueprints/PlayerControllers/PC_Game` _returnvalue_2 :!pure true)))))

(fn `SetupController`
  (params (PlayerCount :type Integer))
  (bind _game_instance (`self.Game Instance`))
  (`GameplayStatics.RemovePlayer` (`GameplayStatics.GetPlayerController` 0))
  (for _index (range PlayerCount)
    (bind _returnvalue (select `int` _index :`0` (`/Game/c013265l/Blueprints/GameInstances/GameInstance.Player0_data` _game_instance) :`1` (`/Game/c013265l/Blueprints/GameInstances/GameInstance.Player1_data` _game_instance) :`2` (`/Game/c013265l/Blueprints/GameInstances/GameInstance.Player2_data` _game_instance) :`3` (`/Game/c013265l/Blueprints/GameInstances/GameInstance.Player3_data` _game_instance)))
    (bind ((`PlayerID_2_B9C8EF28415CAA77CC6887A2B3E5FC49` _playerid) (`PlayerClass_13_AB63BDD64175B900ED43C68475968EA3` _playerclass) (`IsActive_19_07E58887427E7C144A22AE87F1E11D74` _isactive)) (break `/Game/c013265l/Structs/S_PlayerData` _returnvalue))
    (if _isactive
      (bind _returnvalue_2 (`GameplayStatics.CreatePlayer` _playerid))
      (message `/Game/c013265l/Blueprints/Interfaces/BPI_Teams.I_SetPlayerData` _returnvalue_2 _returnvalue)
      (`self.AddToTeamLists` (cast `/Game/c013265l/Blueprints/PlayerControllers/PC_Game` _returnvalue_2 :!pure true)))))

(fn `Spawn Characters`
  (for _array_element (`self.PlayerControllers`)
    (bind _playerdata (message `/Game/c013265l/Blueprints/Interfaces/BPI_Teams.I_GetPlayerData` _array_element))
    (bind ((`PlayerClass_13_AB63BDD64175B900ED43C68475968EA3` _playerclass) (`TeamID_16_C95AF1994DF53F697565858AC86BB26E` _teamid)) (break `/Game/c013265l/Structs/S_PlayerData` _playerdata))
    (bind _returnvalue (`|SpawnActorFromClass` _playerclass (`self.GetTransform` (`self.SelectPlayerSpawn` _teamid)) "AdjustIfPossibleButAlwaysSpawn" "OverrideRootScale" null null))
    (bind _aspawn (cast `Pawn` _returnvalue :!pure true))
    (`Controller.Possess` _array_element _aspawn)
    (message `/Game/c013265l/Blueprints/Interfaces/BPI_PawnCommunication.I_SetPawnTeam` _aspawn _teamid)
    (`PlayerController.SetViewTargetWithBlend` _array_element (`self.MapCam`) 0.0 "VTBlend_Linear" 0.0 false)))

(fn `Spawn Flags`
  (returns (Flags :type "Array of /Game/b017383l/CTF/BP_Flag Object Reference"))
  (bind _outactors (`GameplayStatics.GetAllActorsOfClass` "/Game/b017383l/CTF/BP_FlagSpawn.BP_FlagSpawn_C"))
  (for _array_element _outactors
    (`/Engine/EditorBlueprintResources/StandardMacros.FlipFlop`
      (:`A`
        (bind _returnvalue (`self.GetTransform` _array_element))
        (bind _returnvalue_2 (`|SpawnActorFromClass` "/Game/b017383l/CTF/BP_Flag.BP_Flag_C" _returnvalue "AlwaysSpawn" "OverrideRootScale" null null))
        (message `/Game/c013265l/Blueprints/Interfaces/BPI_Teams.I_SetTeam` _returnvalue_2 "NewEnumerator1"))
      (:`B`
        (bind _returnvalue_3 (`|SpawnActorFromClass` "/Game/b017383l/CTF/BP_Flag.BP_Flag_C" _returnvalue "AlwaysSpawn" "OverrideRootScale" null null))
        (message `/Game/c013265l/Blueprints/Interfaces/BPI_Teams.I_SetTeam` _returnvalue_3 "NewEnumerator2")
        (`KismetArrayLibrary.Array_Add` (`self.Flags`) _returnvalue_3)
        (return)))))

(fn `UserConstructionScript`)
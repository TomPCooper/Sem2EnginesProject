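; Flag spawn point for a Capture the Flag mode, tagged with a Team that it exposes through the I_GetTeam interface.
; It caches the game mode on BeginPlay, and when a Pawn overlaps its Sphere it passes that pawn and itself to GM_Flag through IFlagOverlap.
; All flag rules are left to the game mode, and the I_GetPlayerData implementation is an empty stub.
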(event `self.ReceiveBeginPlay`
  (set `self.Game Mode` (`GameplayStatics.GetGameMode`))
  (bind _teamid (`/Game/c013265l/Blueprints/Interfaces/BPI_Teams.I_GetTeam`))
  (set `self.Team` _teamid))

(event `self.Sphere.OnComponentBeginOverlap`
  (params (OverlappedComponent :type "PrimitiveComponent Object Reference") (OtherActor :type "Actor Object Reference") (OtherComp :type "PrimitiveComponent Object Reference") (OtherBodyIndex :type Integer) (bFromSweep :type Boolean) (SweepResult :type "HitResult Structure (by ref)"))
  (bind _aspawn (cast `Pawn` OtherActor))
  (bind _asgm_flag (cast `/Game/b017383l/CTF/GM_Flag` (`self.Game Mode`)))
  (`self.I_FlagOverlap` _asgm_flag _aspawn self))

(fn `I_GetPlayerData`
  (returns (PlayerData :type "/Game/c013265l/Structs/S_PlayerData Structure"))
  (return))

(fn `I_GetTeam`
  (returns (TeamID :type "/Game/c013265l/Gameplay/Enum_Teams Enum"))
  (return (`self.Team`)))

(fn `UserConstructionScript`)
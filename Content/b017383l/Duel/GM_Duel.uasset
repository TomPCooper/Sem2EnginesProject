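; Game mode for a local two-player duel, scored by kills against a countdown.
; It creates players from GameInstance data, assigns alternating teams, spawns pawns at random matching team starts and points their views at a shared map camera.
; Game state change events drive pre-game, timed play and post-game phases.
; Deaths score for the opposing team and trigger delayed respawns, until the kill limit or timeout brings up the results screen.
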(event `self.ReceiveBeginPlay`
  ;[1 1 1] Start Game
  (set `self.GameInstance` (cast `/Game/c013265l/Blueprints/GameInstances/GameInstance` (`GameplayStatics.GetGameInstance`) :!pure true))
  (bind _returnvalue (`GameplayStatics.GetActorOfClass` "/Game/c013265l/Blueprints/BP_Camera.BP_Camera_C"))
  (set `self.MapCamera` _returnvalue)
  (`self.Init`))

(event `Init`
  ;[1 1 1] Initiate
  (`self.SetUpController`)
  (`self.SpawnCharacters`)
  (`self.BindToGameState`)
  (`/Game/c013265l/Blueprints/PlayerControllers/PC_Game.Init` (`self.GamePlayControllers`))
  (`self.SetScore0`)
  (`self.Setup Game UI`)
  (`KismetSystemLibrary.Delay` 2.0)
  (`/Game/c013265l/Blueprints/GameStates/GS_GameStateBase.UpdateState` (`self.GS_GameState`) "NewEnumerator1" "NewEnumerator4"))

(event `BindToGameState`
  ;[1 1 1] Game State
  (bind _output_get (set `self.GS_GameState` (cast `/Game/c013265l/Blueprints/GameStates/GS_GameStateBase` (`GameplayStatics.GetGameState`) :!pure true)))
  (add `/Game/c013265l/Blueprints/GameStates/GS_GameStateBase.GameStateChanged` _output_get (`|CreateDelegate` :!event `GameStateChanged`)))

(event `/Game/c013265l/Blueprints/Interfaces/BPI_RoundManagement.I_PlayerDeath`
  (params (TeamID :type "/Game/c013265l/Gameplay/Enum_Teams Enum" :default "NewEnumerator0") (DeadPawn :type "Pawn Object Reference"))
  ;[1 1 1] Player Mechanics
  (`self.AddKill` TeamID)
  (bind _aspc_game (cast `/Game/c013265l/Blueprints/PlayerControllers/PC_Game` (`Pawn.GetController` DeadPawn)))
  (`self.CheckScore`)
  (`KismetSystemLibrary.Delay` 4.0)
  (`self.I_RespawnPlayer` _aspc_game TeamID))

(event `GameStateChanged`
  (params (CurrentGameState :type "/Game/c013265l/Blueprints/Enumerators/E_GameState Enum" :default "NewEnumerator0"))
  ;[1 1 1] Game State
  (switch `/Game/c013265l/Blueprints/Enumerators/E_GameState` CurrentGameState
    (:`NewEnumerator1`
      (`KismetSystemLibrary.Delay` 3.0)
      (`/Game/c013265l/Blueprints/GameStates/GS_GameStateBase.UpdateState` (`self.GS_GameState`) "NewEnumerator2" "NewEnumerator4"))
    (:`NewEnumerator2`
      (`self.TimerOn`))
    (:`NewEnumerator3`
      (`self.Remove Input`)
      (`self.Setup End UI`))))

(event `self.I_RespawnPlayer`
  (params (Controller :type "/Game/c013265l/Blueprints/PlayerControllers/PC_Game Object Reference") (TeamID :type "/Game/c013265l/Gameplay/Enum_Teams Enum" :default "NewEnumerator0"))
  ;[1 1 1] Player Mechanics
  (`self.RespawnPlayer` Controller TeamID))

(event `TimerOn`
  ;[1 1 1] Game State
  (`KismetSystemLibrary.K2_SetTimer` null "Game Timer" 1.0 true))

(event `EndGame`
  ;[1 1 1] EndGame
  (bind _outcome (`self.Check Win`))
  (`/Game/c013265l/Blueprints/GameStates/GS_GameStateBase.UpdateState` (`self.GS_GameState`) "NewEnumerator3" _outcome))

(event `ToMenu`
  ;[1 1 1] EndGame
  (`KismetSystemLibrary.Delay` 2.0)
  (`GameplayStatics.OpenLevel` "Menu_Main"))

(event `self.K2_PostLogin`
  (params (NewPlayer :type "PlayerController Object Reference"))
  ;[1 1 1] Login/Logout Events
  (bind _aspc_game (cast `/Game/c013265l/Blueprints/PlayerControllers/PC_Game` NewPlayer))
  (`KismetArrayLibrary.Array_Add` (`self.GamePlayControllers`) _aspc_game))

(event `self.K2_OnLogout`
  (params (ExitingController :type "Controller Object Reference"))
  ;[1 1 1] Login/Logout Events
  (bind _aspc_game (cast `/Game/c013265l/Blueprints/PlayerControllers/PC_Game` ExitingController))
  (`KismetArrayLibrary.Array_RemoveItem` (`self.GamePlayControllers`) _aspc_game)
  (set `self.Player1` null)
  (set `self.Player2` null))

(fn `Add To Player List`
  (params (GameplayController :type "/Game/c013265l/Blueprints/PlayerControllers/PC_Game Object Reference"))
  (`/Engine/EditorBlueprintResources/StandardMacros.FlipFlop`
    (:`A`
      (set `self.Player1` GameplayController))
    (:`B`
      (set `self.Player2` GameplayController))))

(fn `AddKill`
  (params (`Player Team` :type "/Game/c013265l/Gameplay/Enum_Teams Enum" :default "NewEnumerator0"))
  (switch `/Game/c013265l/Gameplay/Enum_Teams` `Player Team`
    (:`NewEnumerator1`
      (`/Engine/EditorBlueprintResources/StandardMacros.IncrementInt` (`self.Player2_Score`)
        (:`  `
          _)))
    (:`NewEnumerator2`
      (`/Engine/EditorBlueprintResources/StandardMacros.IncrementInt` (`self.Player1_Score`)
        (:`  `
          _))))
  (`self.UI Score Change`))

(fn `CanEndGame`
  (returns (CanEnd :type Boolean))
  (if (or (`self.HasTimeRanOut`) (`self.Score Achieved`))
    (return true)
    (else
      (return false))))

(fn `Check Win`
  (returns (Outcome :type "/Game/c013265l/Blueprints/Enumerators/E_GameOutcomes Enum"))
  (if (> (`self.Player1_Score`) (`self.Player2_Score`))
    (bind _output_get (set `self.Game Results` "NewEnumerator0"))
    (return _output_get)
    (elif (< (`self.Player1_Score`) (`self.Player2_Score`))
      (bind _output_get_2 (set `self.Game Results` "NewEnumerator1"))
      (return _output_get_2)
      (else
        (bind _output_get_3 (set `self.Game Results` "NewEnumerator2"))
        (return _output_get_3)))))

(fn `CheckScore`
  (if (>= (`self.Player1_Score`) 6)
    (set `self.Score Achieved` true :!label _label)
    (`self.CanEndGame`)
    (`self.EndGame`)
    (elif (>= (`self.Player2_Score`) 6)
      (goto _label))))

(fn `ChoosePlayerStart`
  (params (Player :type "Controller Object Reference"))
  (returns (ReturnValue :type "Actor Object Reference"))
  (return null))

(fn `Game Timer`
  (set `self.CurrentTime` (- (`self.CurrentTime`) 1.0))
  (`self.UI Time Change`)
  (if (not (>= (`self.CurrentTime`) 0.0))
    (`KismetSystemLibrary.K2_PauseTimer` null "Game Timer")
    (set `self.HasTimeRanOut` true)
    (bind _canend (`self.CanEndGame`))
    (if _canend
      (set `self.CurrentTime` 0.0)
      (`self.EndGame`))))

(fn `I_GetCharacterStats`
  (returns (CharacterStats :type "/Game/c013265l/Blueprints/StructsData/S_CharacterStats Structure"))
  (return))

(fn `I_GetPlayerData`
  (returns (PlayerData :type "/Game/c013265l/Structs/S_PlayerData Structure"))
  (return))

(fn `I_GetTeam`
  (returns (TeamID :type "/Game/c013265l/Gameplay/Enum_Teams Enum"))
  (return "NewEnumerator0"))

(fn `Remove Input`
  (`/Game/c013265l/Blueprints/FucntionLibraries/BPL_GamePlay.RemoveAllPlayers`))

(fn `RespawnPlayer`
  (params (Controller :type "/Game/c013265l/Blueprints/PlayerControllers/PC_Game Object Reference") (TeamID :type "/Game/c013265l/Gameplay/Enum_Teams Enum" :default "NewEnumerator0"))
  (bind _playerdata (message `/Game/c013265l/Blueprints/Interfaces/BPI_Teams.I_GetPlayerData` Controller))
  (bind ((`PlayerClass_13_AB63BDD64175B900ED43C68475968EA3` _playerclass) (`TeamID_16_C95AF1994DF53F697565858AC86BB26E` _teamid)) (break `/Game/c013265l/Structs/S_PlayerData` _playerdata))
  (bind _returnvalue (`|SpawnActorFromClass` _playerclass (`self.GetTransform` (`self.SelectPlayerStart` _teamid)) "AdjustIfPossibleButAlwaysSpawn" "OverrideRootScale" null null))
  (`Controller.Possess` Controller _returnvalue)
  (message `/Game/c013265l/Blueprints/Interfaces/BPI_PawnCommunication.I_SetPawnTeam` _returnvalue _teamid)
  (message `/Game/c013265l/Blueprints/Interfaces/BPI_PawnCommunication.I_InitialiseUI` _returnvalue)
  (`PlayerController.SetViewTargetWithBlend` Controller (`self.MapCamera`) 0.0 "VTBlend_Linear" 0.0 false))

(fn `SelectPlayerStart`
  (params (TeamID :type "/Game/c013265l/Gameplay/Enum_Teams Enum" :default "NewEnumerator0"))
  (returns (StartActor :type "/Game/c013265l/Gameplay/BP_TeamPlayerStart Object Reference"))
  (locals (L_SpawnPointActors :type "Array of /Game/c013265l/Gameplay/BP_TeamPlayerStart Object Reference"))
  (bind _outactors (`GameplayStatics.GetAllActorsOfClass` "/Game/c013265l/Gameplay/BP_TeamPlayerStart.BP_TeamPlayerStart_C"))
  (for _array_element _outactors
    (bind _teamid (message `/Game/c013265l/Blueprints/Interfaces/BPI_Teams.I_GetTeam` _array_element))
    (if (`|EnumEquality` _teamid TeamID)
      (`KismetArrayLibrary.Array_Add` (`local.L_SpawnPointActors`) _array_element)))
  (if (!= (`KismetArrayLibrary.Array_Length` (`local.L_SpawnPointActors`)) 0)
    (return (`KismetArrayLibrary.Array_Random` (`local.L_SpawnPointActors`)))
    (else
      (bind _returnvalue (`GameplayStatics.GetActorOfClass` "/Game/c013265l/Gameplay/BP_TeamPlayerStart.BP_TeamPlayerStart_C"))
      (return _returnvalue))))

(fn `SetScore0`
  (set `self.Player1_Score` 0)
  (set `self.Player2_Score` 0)
  (set `self.CurrentTime` (`self.FinalTime`))
  (set `self.HasTimeRanOut` false))

(fn `Setup End UI`
  (`WidgetLayoutLibrary.RemoveAllWidgets`)
  (bind _returnvalue (`|CreateWidget` "/Game/b017383l/Duel/UI_DuelEnd.UI_DuelEnd_C"))
  (set `self.End UI` _returnvalue)
  (`TextBlock.SetText` (`/Game/b017383l/Duel/UI_DuelEnd.TextAScore` (`self.End UI`)) (`KismetTextLibrary.Conv_StringToText` (`KismetStringLibrary.Concat_StrStr` "Player 1 Score: " (`KismetStringLibrary.Conv_IntToString` (`self.Player1_Score`)))))
  (`TextBlock.SetText` (`/Game/b017383l/Duel/UI_DuelEnd.TextBScore` (`self.End UI`)) (`KismetTextLibrary.Conv_StringToText` (`KismetStringLibrary.Concat_StrStr` "Player 2 Score: " (`KismetStringLibrary.Conv_IntToString` (`self.Player2_Score`)))))
  (add `Button.OnClicked` (`/Game/b017383l/Duel/UI_DuelEnd.ButtonToMenu` (`self.End UI`)) (`|CreateDelegate` :!event `ToMenu`))
  (if (`|EnumEquality` (`self.Game Results`) "NewEnumerator0")
    (`TextBlock.SetText` (`/Game/b017383l/Duel/UI_DuelEnd.TextWinningTeam` (`self.End UI`)) "Player 1 Wins!")
    (elif (`|EnumEquality` (`self.Game Results`) "NewEnumerator1")
      (`TextBlock.SetText` (`/Game/b017383l/Duel/UI_DuelEnd.TextWinningTeam` (`self.End UI`)) "Player 2 Wins!")
      (else
        (`TextBlock.SetText` (`/Game/b017383l/Duel/UI_DuelEnd.TextWinningTeam` (`self.End UI`)) "It's A Draw!"))))
  (`UserWidget.AddToViewport` (`self.End UI`) 0))

(fn `Setup Game UI`
  (bind _returnvalue (`|CreateWidget` "/Game/b017383l/Duel/UI_Duel.UI_Duel_C"))
  (bind _output_get (set `self.Game UI` _returnvalue))
  (`Widget.SetVisibility` _output_get "Visible")
  (`UserWidget.AddToViewport` (`self.Game UI`) 0)
  (`self.UI Time Change`)
  (`self.UI Score Change`))

(fn `SetUpController`
  (bind _gameinstance (`self.GameInstance`))
  (`GameplayStatics.RemovePlayer` (`GameplayStatics.GetPlayerController` 0))
  (for _index (range 2)
    (bind _returnvalue (select `int` _index :`0` (`/Game/c013265l/Blueprints/GameInstances/GameInstance.Player0_data` _gameinstance) :`1` (`/Game/c013265l/Blueprints/GameInstances/GameInstance.Player1_data` _gameinstance)))
    (bind (_playerid _playername _playerclass _teamid _isactive) (break `/Game/c013265l/Structs/S_PlayerData` _returnvalue))
    (if _isactive
      (bind _returnvalue_2 (`GameplayStatics.CreatePlayer` _playerid))
      (message `/Game/c013265l/Blueprints/Interfaces/BPI_Teams.I_SetPlayerData` _returnvalue_2 _returnvalue)
      (`/Engine/EditorBlueprintResources/StandardMacros.FlipFlop`
        (:`A`
          (message `/Game/c013265l/Blueprints/Interfaces/BPI_Teams.I_SetTeam` _returnvalue_2 "NewEnumerator1"))
        (:`B`
          (message `/Game/c013265l/Blueprints/Interfaces/BPI_Teams.I_SetTeam` _returnvalue_2 "NewEnumerator2")))
      (`self.Add To Player List` (cast `/Game/c013265l/Blueprints/PlayerControllers/PC_Game` _returnvalue_2 :!pure true)))))

(fn `SpawnCharacters`
  (for _array_element (`self.GamePlayControllers`)
    (bind _playerdata (message `/Game/c013265l/Blueprints/Interfaces/BPI_Teams.I_GetPlayerData` _array_element))
    (bind ((`PlayerClass_13_AB63BDD64175B900ED43C68475968EA3` _playerclass) (`TeamID_16_C95AF1994DF53F697565858AC86BB26E` _teamid)) (break `/Game/c013265l/Structs/S_PlayerData` _playerdata))
    (bind _returnvalue (`|SpawnActorFromClass` _playerclass (`self.GetTransform` (`self.SelectPlayerStart` _teamid)) "AdjustIfPossibleButAlwaysSpawn" "OverrideRootScale" null null))
    (`Controller.Possess` _array_element _returnvalue)
    (message `/Game/c013265l/Blueprints/Interfaces/BPI_PawnCommunication.I_SetPawnTeam` _returnvalue _teamid)
    (message `/Game/c013265l/Blueprints/Interfaces/BPI_PawnCommunication.I_InitialiseUI` _returnvalue)
    (`PlayerController.SetViewTargetWithBlend` _array_element (`self.MapCamera`) 0.0 "VTBlend_Linear" 0.0 false)))

(fn `UI Score Change`
  (`TextBlock.SetText` (`/Game/b017383l/Duel/UI_Duel.TextAScore` (`self.Game UI`)) (`KismetTextLibrary.Conv_IntToText` (`self.Player1_Score`)))
  (`TextBlock.SetText` (`/Game/b017383l/Duel/UI_Duel.TextBScore` (`self.Game UI`)) (`KismetTextLibrary.Conv_IntToText` (`self.Player2_Score`))))

(fn `UI Time Change`
  (`TextBlock.SetText` (`/Game/b017383l/Duel/UI_Duel.Time` (`self.Game UI`)) (`KismetTextLibrary.Conv_DoubleToText` (`self.CurrentTime`) "HalfToEven")))

(fn `UserConstructionScript`)
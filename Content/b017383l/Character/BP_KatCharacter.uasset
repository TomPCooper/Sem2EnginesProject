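; Playable Kat character Blueprint that implements a team-aware basic attack and three abilities.
; On init it caches its team, then passes it to the projectile, web trap and ultimate stun actors it spawns.
; Web traps are tracked in an array that destroys the oldest beyond three.
; The second ability instantly heals, while the ultimate spawns a stun actor and holds an InUltimate flag until a timer clears it.
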(event `self.ReceiveBeginPlay`
  ;[1 1 1] Init
  (`self.CharaInit`))

(event `CharaInit`
  ;[1 1 1] Init
  (`KismetArrayLibrary.Array_Clear` (`self.Current Traps`))
  (bind _teamid (`self.I_GetTeam`))
  (set `self.PlayerTeam` _teamid))

(event `self.FireBasicAttack`
  ;[1 1 1] Basic Attack (Using A018745l Projectiles)
  (`|SpawnActorFromClass` "/Game/A018745l/Basic_Projectile.Basic_Projectile_C" (`SceneComponent.K2_GetComponentToWorld` (`self.Fire Direction`)) "Undefined" "OverrideRootScale" null (`self.GetController`) self (`self.PlayerTeam`) self))

(event `self.FireAbility1`
  ;[1 1 1] Ability 1 - Web Trap
  (`KismetSystemLibrary.PrintString` "trap spawning")
  (bind _returnvalue (`|SpawnActorFromClass` "/Game/b017383l/Character/BP_WebTrap.BP_WebTrap_C" (`KismetMathLibrary.MakeTransform` (`SceneComponent.K2_GetComponentLocation` (`self.Drop Direction`))) "Undefined" "OverrideRootScale" null (`self.PlayerTeam`) (`self.GetController`) null))
  (`KismetArrayLibrary.Array_Add` (`self.Current Traps`) _returnvalue)
  (`self.Check Array`))

(event `self.FireAbility2`
  ;[1 1 1] Ability 2 - Instant Heal
  (`self.ModifyHealth` 20.0 true))

(event `self.FireAbility3`
  ;[1 1 1] Ability 3
  (set `self.InUltimate` true)
  (`KismetSystemLibrary.K2_SetTimerDelegate` (delegate `Ultimate End`) 10.0)
  (`|SpawnActorFromClass` "/Game/b017383l/Character/BP_UltiStun.BP_UltiStun_C" (`KismetMathLibrary.MakeTransform` (`SceneComponent.K2_GetComponentLocation` (`self.Drop Direction`))) "Undefined" "OverrideRootScale" null (`self.PlayerTeam`) null))

(event `Ultimate End`
  ;[1 1 1] Ability 3
  (set `self.InUltimate` false))

(fn `Check Array`
  (locals (`Removeable Trap` :type "/Game/b017383l/Character/BP_WebTrap Object Reference"))
  (bind _current_traps (`self.Current Traps`))
  (if (> (`KismetArrayLibrary.Array_Length` (`self.Current Traps`)) 3)
    (set `local.Removeable Trap` (`|GetArrayItem` _current_traps))
    (`KismetArrayLibrary.Array_Remove` _current_traps)
    (`self.K2_DestroyActor` (`local.Removeable Trap`))))

(fn `UserConstructionScript`
  (`parent.UserConstructionScript`))
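; BP_Trap is a single-use trap actor that damages overlapping actors from opposing teams.
; On overlap it reads the other actor's TeamID through a player-data interface message and compares it with OwnerTeam.
; A mismatch applies TrapDamage as BP_StandardDamage and destroys the trap.
; Its own GetTeam interface returns a fixed enum value rather than OwnerTeam, and its player-data getter returns nothing.
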(event `self.ReceiveActorBeginOverlap`
  (params (OtherActor :type "Actor Object Reference"))
  ;[1 1 1] On Overlap
  (bind _output_get (set `self.OverlappedPawn` OtherActor))
  (bind _playerdata (message `/Game/c013265l/Blueprints/Interfaces/BPI_Teams.I_GetPlayerData` _output_get))
  (if (`|EnumInequality` (`.TeamID_16_C95AF1994DF53F697565858AC86BB26E` (break `/Game/c013265l/Structs/S_PlayerData` _playerdata)) (`self.OwnerTeam`))
    (`GameplayStatics.ApplyDamage` (`self.OverlappedPawn`) (`self.TrapDamage`) null null "/Game/c013265l/Blueprints/DamageTypes/BP_StandardDamage.BP_StandardDamage_C")
    (`self.K2_DestroyActor`)))

(fn `I_GetPlayerData`
  (returns (PlayerData :type "/Game/c013265l/Structs/S_PlayerData Structure"))
  (return))

(fn `I_GetTeam`
  (returns (TeamID :type "/Game/c013265l/Gameplay/Enum_Teams Enum"))
  (return "NewEnumerator0"))

(fn `UserConstructionScript`)
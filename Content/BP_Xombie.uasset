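; BP_Xombie is a zombie enemy that takes damage and reports its death to the game mode.
; AnyDamage passes the damage and instigator to the Health function, which either heals up to MaxHealth or subtracts from CharacterStats.CurrentHealth.
; The result stays in a local and is never written back to CharacterStats.
; At zero or below, Health sends IOnZombieDeathMessage with the attacker to the game mode.
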(event `self.ReceiveAnyDamage`
  (params (Damage :type "Float (single-precision)") (DamageType :type "DamageType Object Reference") (InstigatedBy :type "Controller Object Reference") (DamageCauser :type "Actor Object Reference"))
  (`self.Health` Damage false InstigatedBy))

(fn `Health`
  (params (`Health Modify` :type "Float (double-precision)") (IsHealing :type Boolean) (AttackerRef :type "Controller Object Reference"))
  (locals (L_CurrentHealth :type "Float (double-precision)"))
  (bind ((`MaxHealth_2_901ADD2C4C74E5308EC359A5539E7D95` _maxhealth) (`CurrentHealth_4_E7CB1D7448D4E0198F1304A316B5B9E5` _currenthealth)) (break `/Game/c013265l/Blueprints/StructsData/S_CharacterStats` (`self.CharacterStats`)))
  (bind _returnvalue (+ _currenthealth `Health Modify`))
  (if IsHealing
    (if (> _returnvalue _maxhealth)
      (set `local.L_CurrentHealth` _maxhealth)
      (else
        (set `local.L_CurrentHealth` _returnvalue)))
    (else
      (set `local.L_CurrentHealth` (- _currenthealth `Health Modify`))))
  (if (<= (`local.L_CurrentHealth`) 0.0)
    (message `/Game/BPI_Zombies.I_On Zombie Death` (`GameplayStatics.GetGameMode`) AttackerRef)))

(fn `UserConstructionScript`)